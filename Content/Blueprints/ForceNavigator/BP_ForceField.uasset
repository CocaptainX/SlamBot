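; BP_ForceField is an actor that displays a force field as a flattened component with adjustable position, size and visibility.
; An Update event stores Location and Magnitude, moves the ForceField component to that relative location and scales its X and Y by Magnitude with a thin fixed Z.
; The same event sets whether the actor is hidden in game, and BeginPlay calls it with the stored values and visibility on.
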(event `self.ReceiveBeginPlay`
  (`self.Update` (`self.Location`) (`self.Magnitude`)))

(event `Update`
  (params (Location :type "Vector Structure") (Magnitude :type "Float (double-precision)") (IsVisible :type Boolean :default true))
  (bind _output_get (set `self.Location` Location))
  (`SceneComponent.K2_SetRelativeLocation` (`self.ForceField`) _output_get false false)
  (bind _output_get_2 (set `self.Magnitude` Magnitude))
  (`SceneComponent.SetRelativeScale3D` (`self.ForceField`) (`KismetMathLibrary.MakeVector` _output_get_2 _output_get_2 0.1))
  (`self.SetActorHiddenInGame` (not IsVisible)))

(fn `UserConstructionScript`)