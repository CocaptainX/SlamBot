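; BP_ForceNavigator keeps timed, grouped point force fields and computes a combined push vector away from them.
; Each Tick it ages and purges fields, then sums forces at LocationIndicator's relative location, each falling off with inverse distance.
; Debug mode shows the result as a scaled arrow, with optional BP_ForceField actors mirroring the field array by index.
; MoveForceFieldsBy shifts only those visuals, as its field-data update is unwired.
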(event `Initialize`
  (params (Debug :type Boolean))
  ;[1 1 1] Show or hide the push direction based on debug mode
  (bind _output_get (set `self.Debug` Debug))
  (`SceneComponent.SetHiddenInGame` (`self.PushDirectionIndicator`) (not _output_get) false))

(event `self.ReceiveTick`
  (params (DeltaSeconds :type "Float (single-precision)"))
  ;[1 1 1] Update force field lifetimes and purge dead ones
  (`self.UpdateLifetimes` DeltaSeconds)
  (`self.PurgeExpiredForceFields`)
  ;[1 1 1] Calculate the combined push force
  (bind _pushforce (`self.CalculateCombinedPushForce` (`self.ForceFields`)))
  (bind _output_get (set `self.PushForce` _pushforce))
  ;[1 1 1] Visualize the push force if debugging is enabled
  (if (`self.Debug`)
    (`self.UpdatePushForceArrow` _output_get)))

(fn `CalculateCombinedPushForce`
  (params (ForceFields :type "Array of /Game/Blueprints/ForceNavigator/ST_ForceField Structure"))
  (returns (PushForce :type "Vector Structure"))
  (locals (PushForceAccumulator :type "Vector Structure"))
  (bind _pushforceaccumulator (`local.PushForceAccumulator`))
  (for _array_element ForceFields
    (bind (_location _magnitude) (break `/Game/Blueprints/ForceNavigator/ST_ForceField` _array_element))
    (bind _fieldforce (`self.CalculateFieldForce` (`SceneComponent.RelativeLocation` (`self.LocationIndicator`)) _location _magnitude))
    (set `local.PushForceAccumulator` (+ _fieldforce _pushforceaccumulator)))
  (return _pushforceaccumulator))

(fn `CalculateFieldForce`
  (params (ReferenceLocation :type "Vector Structure") (ForceLocation :type "Vector Structure") (Magnitude :type "Float (double-precision)"))
  (returns (FieldForce :type "Vector Structure"))
  (bind _returnvalue (- ReferenceLocation ForceLocation))
  (return (* (`KismetMathLibrary.Normal` _returnvalue) (* (/ Magnitude (`KismetMathLibrary.VSize` _returnvalue)) 100.0))))

(fn `ClearByGroupId`
  (params (GroupId :type Integer))
  (locals (InitialForceFieldCount :type Integer))
  (bind _forcefields (`self.ForceFields`))
  (set `local.InitialForceFieldCount` (`KismetArrayLibrary.Array_Length` _forcefields))
  (bind (_arrayindex _arrayelement) (`/Engine/EditorBlueprintResources/StandardMacros.ReverseForEachLoop` _forcefields)
    (:`LoopBody`
      (if (== (`.GroupId_12_4E50493742A47934C08CE0959F7FD154` (break `/Game/Blueprints/ForceNavigator/ST_ForceField` _arrayelement)) GroupId)
        (`self.RemoveForceFieldByIndex` _arrayindex)))))

(fn `CreateForceField`
  (params (Location :type "Vector Structure") (Magnitude :type "Float (double-precision)") (Lifetime :type "Float (double-precision)") (GroupId :type Integer))
  (`|ExecutionSequence`
    (:`then_0`
      ;[1 1 1] Create the internal representation used for calculations
      (`KismetArrayLibrary.Array_Add` (`self.ForceFields`) (make `/Game/Blueprints/ForceNavigator/ST_ForceField` Location Magnitude Lifetime Lifetime GroupId)))
    (:`then_1`
      ;[1 1 1] Also create the visual representation if debug mode and visualization are enabled
      (if (and (`self.Debug`) (`self.VisualizeForceFields`))
        (bind _returnvalue (`|SpawnActorFromClass` "/Game/Blueprints/ForceNavigator/BP_ForceField.BP_ForceField_C" (`KismetMathLibrary.MakeTransform` Location) "Undefined" "OverrideRootScale" null Magnitude))
        (`SceneComponent.K2_AttachToComponent` (`/Game/Blueprints/ForceNavigator/BP_ForceField.ForceField` _returnvalue) (`self.Scene`) "None" "KeepRelative" "KeepRelative" "KeepRelative" true)
        (`KismetArrayLibrary.Array_Add` (`self.ForceFieldVisuals`) _returnvalue)))))

(fn `MoveForceFieldsBy`
  (params (DeltaPosition :type "Vector Structure"))
  (`|ExecutionSequence`
    (:`then_1`
      ;[1 1 1] Also update the visual location if debug mode and visualization are enabled
      (if (and (`self.Debug`) (`self.VisualizeForceFields`))
        (for _array_element (`self.ForceFieldVisuals`)
          (`self.K2_SetActorLocation` _array_element (- (`self.K2_GetActorLocation` _array_element) DeltaPosition) false false))))))

(fn `PurgeExpiredForceFields`
  ;[1 1 1] Detect and remove force fields that have expired
  (bind (_arrayindex _arrayelement) (`/Engine/EditorBlueprintResources/StandardMacros.ReverseForEachLoop` (`self.ForceFields`))
    (:`LoopBody`
      (if (<= (`.LifetimeRemaining_9_E0458CDD4D944C767989E8907F06B35F` (break `/Game/Blueprints/ForceNavigator/ST_ForceField` _arrayelement)) 0.0)
        (`self.RemoveForceFieldByIndex` _arrayindex)))))

(fn `RemoveForceFieldByIndex`
  (params (Index :type Integer))
  (bind _forcefieldvisuals (`self.ForceFieldVisuals`))
  ;[1 1 1] Remove the force field from the array
  (`KismetArrayLibrary.Array_Remove` (`self.ForceFields`) Index)
  ;[1 1 1] Also remove the debug visual if debug mode and visualization is enabled
  (if (and (`self.Debug`) (`self.VisualizeForceFields`))
    (`self.K2_DestroyActor` (`KismetArrayLibrary.Array_Get` _forcefieldvisuals Index))
    (`KismetArrayLibrary.Array_Remove` _forcefieldvisuals Index)))

(fn `UpdateLifetimes`
  (params (DeltaSeconds :type "Float (double-precision)"))
  (for (_array_element _array_index) (`self.ForceFields`)
    (bind _structout (setmembers `/Game/Blueprints/ForceNavigator/ST_ForceField` :`StructRef` _array_element :`LifetimeRemaining` (`KismetMathLibrary.FMax` (- (`.LifetimeRemaining_9_E0458CDD4D944C767989E8907F06B35F` (break `/Game/Blueprints/ForceNavigator/ST_ForceField` _array_element)) DeltaSeconds))))
    (`KismetArrayLibrary.Array_Set` (`self.ForceFields`) _array_index _structout)))

(fn `UpdatePushForceArrow`
  (params (PushForce :type "Vector Structure"))
  (locals (UnitScale :type "Float (double-precision)" :default 0.1))
  (bind _pushdirectionindicator (`self.PushDirectionIndicator`))
  (bind _unitscale (`local.UnitScale`))
  (`SceneComponent.K2_SetRelativeRotation` _pushdirectionindicator (`KismetMathLibrary.MakeRotationFromAxes` PushForce (0.0 1.0 0.0) (0.0 0.0 1.0)) false false)
  (`SceneComponent.SetRelativeScale3D` _pushdirectionindicator (`KismetMathLibrary.MakeVector` (* (`KismetMathLibrary.VSize` PushForce) _unitscale) _unitscale _unitscale)))

(fn `UserConstructionScript`)