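; Simulated tracked robot that turns longitudinal and turn speed commands into differential drive for two child-actor treads.
; Each Tick it sends left and right speeds to the treads, then steps Odometry using their reported speeds and the tread spacing measured at BeginPlay.
; The odometry estimate moves an OdometryPose component for visualization.
; GetCurrentSpeed separately reports forward speed from chassis physics velocity.
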(event EventSetLongitudinalSpeed
  (params (Speed :type Float%20%28single-precision%29))
  (|CallParentFunction Speed))

(event EventSetTurnSpeed
  (params (Speed :type Float%20%28single-precision%29))
  (|CallParentFunction Speed))

(event EventBeginPlay
  (|CallParentFunction)
  (Utilities|FlowControl|Sequence
    (:then_0
      ;[1 1 1] Get references to tread components
      (bind _asbp_robot_tread_right (Utilities|Casting|CastToBP_Robot_TreadRight (Variables|/Script/Engine.ChildActorComponent|GetChildActor (Variables|Default|GetRightTreadActor))))
      (Variables|Runtime|SetRightTread _asbp_robot_tread_right))
    (:then_1
      (bind _asbp_robot_tread_right_2 (Utilities|Casting|CastToBP_Robot_TreadRight (Variables|/Script/Engine.ChildActorComponent|GetChildActor (Variables|Default|GetLeftTreadActor))))
      (Variables|Runtime|SetLeftTread _asbp_robot_tread_right_2))
    (:then_2
      (CallFunction|UpdateDistanceBetweenTreads))))

(event EventTick
  (params (DeltaSeconds :type Float%20%28single-precision%29))
  (Utilities|FlowControl|Sequence
    (:then_0
      ;[1 1 1] Update tread speeds
      (bind (_lefttreadspeed _righttreadspeed) (CallFunction|CalculateDifferentialDrive (Variables|Default|GetLongitudinalSpeed) (Variables|Default|GetTurnSpeed)))
      (Utilities|FlowControl|Sequence
        (:then_0
          (Default|SetSpeed (Variables|Runtime|GetLeftTread) _lefttreadspeed))
        (:then_1
          (Default|SetSpeed (Variables|Runtime|GetRightTread) _righttreadspeed))))
    (:then_1
      ;[1 1 1] Update and visualize odometry
      (CallFunction|StepOdometry)
      (CallFunction|VisualizeOdometry))))

(fn ConstructionScript)

(fn CalculateDifferentialDrive
  (params (LongitudinalSpeed :type Float%20%28single-precision%29) (TurnSpeed :type Float%20%28single-precision%29))
  (bind _returnvalue (* TurnSpeed 1.0))
  (bind _returnvalue_2 (- LongitudinalSpeed _returnvalue))
  (bind _returnvalue_3 (+ LongitudinalSpeed _returnvalue))
  (LocalVariables|SetMaxTreadSpeed (Math|Float|Max(Float) _returnvalue_3 _returnvalue_2))
  (return _returnvalue_3 _returnvalue_2))

(fn GetCurrentSpeed
  (bind _chassis (Variables|Default|GetChassis))
  (bind _returnvalue (Physics|GetPhysicsLinearVelocity _chassis "None"))
  (return (/ (Math|Vector|DotProduct _returnvalue (Math|Transform|TransformDirection (Transformation|GetWorldTransform _chassis) "1.000000, 0, 0")) 1e+02)))

(fn StepOdometry
  (bind _speedmeterspersecond (Default|GetTreadSpeed (Variables|Runtime|GetLeftTread)))
  (bind _speedmeterspersecond_2 (Default|GetTreadSpeed (Variables|Runtime|GetRightTread)))
  (Default|Step (Variables|Default|GetOdometry) _speedmeterspersecond _speedmeterspersecond_2 (Variables|Runtime|GetDistanceBetweenTreads)))

(fn VisualizeOdometry
  (bind _odometry (Variables|Default|GetOdometry))
  (bind _position (Variables|/Game/Blueprints/Robot/BP_Robot_Odometry.BP_Robot_Odometry_C|GetPosition _odometry))
  (Transformation|SetRelativeLocationAndRotation (Variables|Default|GetOdometryPose) (Math|Vector|MakeVector (.x _position) (.y _position) (.z (Variables|/Script/Engine.SceneComponent|GetRelativeLocation (Variables|Default|GetChassis)))) (Variables|/Game/Blueprints/Robot/BP_Robot_Odometry.BP_Robot_Odometry_C|GetRotation _odometry) false true))

(fn GetDistanceBetweenTreads
  (return (Math|Vector|VectorLength (- (Transformation|GetWorldLocation (VehicleSound|GetRootComponent (Variables|Runtime|GetLeftTread))) (Transformation|GetWorldLocation (VehicleSound|GetRootComponent (Variables|Runtime|GetRightTread)))))))

(fn UpdateDistanceBetweenTreads
  (bind _distancebetweentreads (CallFunction|GetDistanceBetweenTreads))
  (bind _output_get (Variables|Runtime|SetDistanceBetweenTreads _distancebetweentreads))
  (Development|PrintText (Utilities|Text|FormatText "Distance: {distance}" (Utilities|Text|ToText(Float) _output_get "HalfToEven"))))