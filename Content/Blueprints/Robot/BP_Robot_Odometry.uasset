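; Robot odometry Blueprint that estimates the pose of a treaded, differential-drive robot by dead reckoning.
; Step converts left and right tread speeds into centimeters travelled over the world delta time, then derives center distance and heading change from tread spacing.
; It advances Position along the previous yaw before updating Rotation, keeping the pose planar with zero Z, pitch and roll.
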(fn `Step`
  (params (LeftSpeed :type "Float (double-precision)") (RightSpeed :type "Float (double-precision)") (DistanceBetweenTreads :type "Float (double-precision)"))
  (locals (LeftDistanceTravelledCentimeters :type "Float (double-precision)") (RightDistanceTravelledCentimeter :type "Float (double-precision)") (CenterDistanceTravelledCentimeter :type "Float (double-precision)") (HeadingDifferenceRadians :type "Float (double-precision)"))
  (bind (_position_x _position_y) (`KismetMathLibrary.BreakVector` (`self.Position`)))
  (bind (_rotation_roll _rotation_pitch _rotation_yaw) (`KismetMathLibrary.BreakRotator` (`self.Rotation`)))
  (bind (_rotation_roll_2 _rotation_pitch_2 _rotation_yaw_2) (`KismetMathLibrary.BreakRotator` (`self.Rotation`)))
  (bind (_rotation_roll_3 _rotation_pitch_3 _rotation_yaw_3) (`KismetMathLibrary.BreakRotator` (`self.Rotation`)))
  (`|ExecutionSequence`
    (:`then_0`
      ;[1 1 1] Calculate left, right and center distances travelled
      (set `local.LeftDistanceTravelledCentimeters` (* (* LeftSpeed (`GameplayStatics.GetWorldDeltaSeconds`)) 100.0)))
    (:`then_1`
      (set `local.RightDistanceTravelledCentimeter` (* (* RightSpeed (`GameplayStatics.GetWorldDeltaSeconds`)) 100.0)))
    (:`then_2`
      (set `local.CenterDistanceTravelledCentimeter` (/ (+ (`local.LeftDistanceTravelledCentimeters`) (`local.RightDistanceTravelledCentimeter`)) 2.0)))
    (:`then_3`
      ;[1 1 1] Calculate heading change
      (set `local.HeadingDifferenceRadians` (/ (- (`local.LeftDistanceTravelledCentimeters`) (`local.RightDistanceTravelledCentimeter`)) DistanceBetweenTreads)))
    (:`then_4`
      ;[1 1 1] Calculate new position
      (set `self.Position` (`KismetMathLibrary.MakeVector` (+ _position_x (* (`local.CenterDistanceTravelledCentimeter`) (`KismetMathLibrary.DegCos` _rotation_yaw_3))) (+ _position_y (* (`local.CenterDistanceTravelledCentimeter`) (`KismetMathLibrary.DegSin` _rotation_yaw_2))))))
    (:`then_5`
      ;[1 1 1] Update rotation
      (set `self.Rotation` (`KismetMathLibrary.MakeRotator` 0.0 0.0 (+ _rotation_yaw (`KismetMathLibrary.RadiansToDegrees` (`local.HeadingDifferenceRadians`))))))))