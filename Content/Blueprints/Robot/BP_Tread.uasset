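; BP_Tread is a physics-driven robot tread with front and rear wheels.
; On BeginPlay it finds the static mesh at the top of its scene attachment chain and binds both wheel constraints between that mesh and the wheels.
; Each tick it torques only the front wheel around the parent mesh's local X axis, scaled by the target speed set through SetSpeed.
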(event `self.ReceiveBeginPlay`
  (`|ExecutionSequence`
    (:`then_0`
      ;[1 1 1] Extract the parent static mesh component to attach to
      (bind _staticmesh (`self.GetParentStaticMesh`))
      (set `self.ParentComponent` _staticmesh))
    (:`then_1`
      ;[1 1 1] Update wheel constraint parents
      (`self.SetParentComponent` (`self.RearWheelConstraint`) (`self.RearWheel`)))
    (:`then_2`
      (`self.SetParentComponent` (`self.FrontWheelConstraint`) (`self.FrontWheel`)))))

(event `self.ReceiveTick`
  (params (DeltaSeconds :type "Float (single-precision)"))
  (`PrimitiveComponent.AddTorque` (`self.FrontWheel`) (* (`KismetMathLibrary.TransformDirection` (`SceneComponent.K2_GetComponentToWorld` (`self.ParentComponent`)) (1.0 0.0 0.0)) (* (`self.TargetSpeed`) 500.0)) "None" false))

(fn `GetParentStaticMesh`
  (returns (StaticMesh :type "StaticMeshComponent Object Reference"))
  (bind _parents (`SceneComponent.GetParentComponents` (`self.Scene`)))
  (bind _asstatic_mesh_component (cast `StaticMeshComponent` (`KismetArrayLibrary.Array_Get` _parents (`KismetArrayLibrary.Array_LastIndex` _parents)))
    (:`then`
      _)
    (:`CastFailed`
      (`KismetSystemLibrary.PrintText` "Getting parent static mesh component failed!" true true (struct :`R` 1.0 :`A` 1.0) 30.0)))
  (return _asstatic_mesh_component))

(fn `SetParentComponent`
  (params (Constraint :type "PhysicsConstraintComponent Object Reference") (Child :type "StaticMeshComponent Object Reference"))
  (`PhysicsConstraintComponent.SetConstrainedComponents` Constraint (`self.ParentComponent`) "None" Child "None"))

(fn `SetSpeed`
  (params (Speed :type "Float (double-precision)"))
  (set `self.TargetSpeed` Speed))

(fn `UserConstructionScript`)