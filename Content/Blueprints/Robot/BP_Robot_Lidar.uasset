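; Simulated spinning 2D lidar for a robot, reporting distance readings around a full revolution.
; Each Tick spins the turret at a set RPM and substeps through every angle step due by the new yaw, keeping sample count independent of frame rate.
; Each step line-traces between min and max range from ScanOrigin, yielding distance and binary signal strength.
; Readings fire LidarMeasurement individually and accumulate until ScanComplete delivers the full list.
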(event `self.ReceiveBeginPlay`
  ;[1 1 1] Calculate the measurement step angle given measurements per revolution
  (set `self.MeasurementStepAngle` (/ 360.0 (`KismetMathLibrary.Conv_IntToDouble` (`self.MeasurementsPerRevolution`)))))

(event `self.ReceiveTick`
  (params (DeltaSeconds :type "Float (single-precision)"))
  (bind _measurementlist (`self.MeasurementList`))
  (bind _performedmeasurementcount (`self.PerformedMeasurementCount`))
  ;[1 1 1] Update turrent rotation
  (bind _turrentangle (`self.UpdateTurrentRotation` DeltaSeconds))
  ;[1 1 1] Calculate expected and required step count
  (bind _expectedmeasurementcount (`self.CalculateExpectedMeasurementCount` _turrentangle))
  (bind _output_get (set `self.ScanSubstepCount` (- _expectedmeasurementcount _performedmeasurementcount)))
  ;[1 1 1] Calculate substep loop indexes and update performed measurement count once complete
  (for _index (range _performedmeasurementcount (+ (`KismetMathLibrary.Min` (- (+ _performedmeasurementcount _output_get) 1) (- (`self.MeasurementsPerRevolution`) 1)) 1))
    ;[1 1 1] Calculate current substep scan angle
    (bind _output_get_2 (set `self.ScanAngle` (* (`KismetMathLibrary.Conv_IntToDouble` _index) (`self.MeasurementStepAngle`))))
    ;[1 1 1] Make the distance measurement and build measurement representation
    (bind (_distance _signalstrength) (`self.MakeDistanceMeasurement` _output_get_2))
    (bind _st_lidarmeasurement (make `/Game/Blueprints/Lidar/ST_LidarMeasurement` _index _output_get_2 _distance _signalstrength))
    ;[1 1 1] Add the measurement to the list of measurements and trigger custom event
    (`KismetArrayLibrary.Array_Add` (`self.MeasurementList`) _st_lidarmeasurement)
    (`self.Event Lidar Measurement` _st_lidarmeasurement))
  ;[1 1 1] Update performed measurement count and trigger scan complete if a rotation was completed
  (if (>= (`KismetArrayLibrary.Array_Length` (`self.MeasurementList`)) (`self.MeasurementsPerRevolution`))
    (set `self.PerformedMeasurementCount` 0)
    (`self.Event Scan Complete` _measurementlist)
    (`KismetArrayLibrary.Array_Clear` _measurementlist)
    (else
      (set `self.PerformedMeasurementCount` _index))))

(event `Event Lidar Measurement`
  (params (Measurement :type "/Game/Blueprints/Lidar/ST_LidarMeasurement Structure")))

(event `Event Scan Complete`
  (params (MeasurementList :type "Array of /Game/Blueprints/Lidar/ST_LidarMeasurement Structure")))

(fn `CalculateExpectedMeasurementCount`
  (params (TurrentAngle :type "Float (double-precision)"))
  (returns (ExpectedMeasurementCount :type Integer))
  ;[1 1 1] Calculates how many lidar measurements should have been made by given turrent angle
  (return (`KismetMathLibrary.FFloor` (* (/ TurrentAngle 360.0) (`KismetMathLibrary.Conv_IntToDouble` (`self.MeasurementsPerRevolution`))))))

(fn `MakeDistanceMeasurement`
  (params (Angle :type "Float (double-precision)"))
  (returns (Distance :type "Float (double-precision)") (SignalStrength :type Integer))
  (locals (DebugTrace :type "EDrawDebugTrace Enum"))
  (bind _scanorigin (`self.ScanOrigin`))
  (bind _returnvalue (`SceneComponent.K2_GetComponentLocation` _scanorigin))
  (bind _returnvalue_2 (`KismetMathLibrary.RotateAngleAxis` (`SceneComponent.GetForwardVector` _scanorigin) Angle (`SceneComponent.GetUpVector` _scanorigin)))
  (if (`self.Debug`)
    (set `local.DebugTrace` "ForDuration")
    (else
      (set `local.DebugTrace` "None")))
  (bind (_outhit _returnvalue_3) (`KismetSystemLibrary.LineTraceSingle` :`Start` (+ (* _returnvalue_2 (`self.LidarSenseMinDistance`)) _returnvalue) :`End` (+ _returnvalue (* _returnvalue_2 (`self.LidarSenseMaxDistance`))) :`TraceChannel` "TraceTypeQuery1" :`bTraceComplex` true :`DrawDebugType` (`local.DebugTrace`) :`DrawTime` 1.0))
  (if _returnvalue_3
    (bind (_bblockinghit _binitialoverlap _time _location _impactpoint _normal _impactnormal _physmat _hitactor _hitcomponent _hitbonename _hititem _faceindex _tracestart) (`GameplayStatics.BreakHitResult` _outhit))
    (return (`KismetMathLibrary.VSize` (- _location _tracestart)) 1)
    (else
      (return (`self.LidarSenseMaxDistance`) 0))))

(fn `UpdateTurrentRotation`
  (params (DeltaSeconds :type "Float (double-precision)"))
  (returns (TurrentAngle :type "Float (double-precision)"))
  (locals (TurrentAngleDiff :type "Float (double-precision)") (IsRotationComplete :type Boolean))
  (bind _turrent (`self.Turrent`))
  (bind (_relativerotation_roll _relativerotation_pitch _relativerotation_yaw) (`KismetMathLibrary.BreakRotator` (`SceneComponent.RelativeRotation` _turrent)))
  (bind _returnvalue (+ _relativerotation_yaw (* (* (/ (`self.TurrentRPM`) 60.0) DeltaSeconds) 360.0)))
  ;[1 1 1] Update turrent angle
  (`SceneComponent.K2_SetRelativeRotation` _turrent (`KismetMathLibrary.MakeRotator` 0.0 0.0 _returnvalue) false false)
  ;[1 1 1] Report turrent angle in the 0..360 degrees range
  (return (+ _returnvalue 180.0)))

(fn `UserConstructionScript`)