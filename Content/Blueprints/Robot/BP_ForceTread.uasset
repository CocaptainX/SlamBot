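; BP_ForceTread is a robot tread that propels itself with physics forces along whatever surface it is touching.
; On each Tread hit, it crosses the hit normal with the tread's local -Y axis to get a drive direction, then applies force at ForceLocation scaled by TargetSpeed.
; SetSpeed sets TargetSpeed, and a debug HitArrow shows the contact point and drive direction, hidden again every Tick.
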(event `self.ReceiveBeginPlay`)

(event `self.ReceiveActorBeginOverlap`
  (params (OtherActor :type "Actor Object Reference")))

(event `self.ReceiveTick`
  (params (DeltaSeconds :type "Float (single-precision)"))
  (`SceneComponent.SetVisibility` (`self.HitArrow`) false false))

(event `self.Tread.OnComponentHit`
  (params (OtherActor :type "Actor Object Reference") (OtherComp :type "PrimitiveComponent Object Reference") (NormalImpulse :type "Vector Structure") (Hit :type "HitResult Structure (by ref)"))
  (bind _hitarrow (`self.HitArrow`))
  (bind _returnvalue (`KismetMathLibrary.Cross_VectorVector` Hit_Normal (`KismetMathLibrary.TransformDirection` (`SceneComponent.K2_GetComponentToWorld` (`self.Tread`)) (0.0 -1.0 0.0))))
  (`|ExecutionSequence`
    (:`then_0`
      (`SceneComponent.K2_SetWorldLocation` _hitarrow Hit_Location false false))
    (:`then_1`
      (`SceneComponent.K2_SetWorldRotation` _hitarrow (`KismetMathLibrary.MakeRotationFromAxes` _returnvalue (0.0 1.0 0.0) (0.0 0.0 1.0)) false false))
    (:`then_2`
      (`PrimitiveComponent.AddForceAtLocation` (`self.Tread`) (* _returnvalue (* (`self.TargetSpeed`) 350.0)) (`SceneComponent.K2_GetComponentLocation` (`self.ForceLocation`)) "None"))
    (:`then_3`
      (`SceneComponent.SetVisibility` (`self.HitArrow`) true false))))

(fn `SetSpeed`
  (params (Speed :type "Float (double-precision)"))
  (set `self.TargetSpeed` Speed))

(fn `UserConstructionScript`)