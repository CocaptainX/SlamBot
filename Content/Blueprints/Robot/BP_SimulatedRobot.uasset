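; Simulated robot that drives on two child-actor treads using differential drive.
; BeginPlay caches both treads, each cast to BP_RightTread, while the speed setters defer to the parent class.
; Each tick it mixes longitudinal and scaled turn speed into left and right tread speeds and sends them to the treads.
; GetCurrentSpeed reports the chassis physics velocity along its forward axis in meters per second.
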(event EventSetLongitudinalSpeed
  (params (Speed :type Float%20%28single-precision%29))
  (|CallParentFunction Speed))

(event EventSetTurnSpeed
  (params (Speed :type Float%20%28single-precision%29))
  (|CallParentFunction Speed))

(event EventBeginPlay
  (|CallParentFunction)
  (Utilities|FlowControl|Sequence
    (:then_0
      ;[1 1 1] Get references to tread components
      (bind _asbp_right_tread (Utilities|Casting|CastToBP_RightTread (Variables|/Script/Engine.ChildActorComponent|GetChildActor (Variables|Default|GetRightTreadActor))))
      (Variables|Runtime|SetRightTread _asbp_right_tread))
    (:then_1
      (bind _asbp_right_tread_2 (Utilities|Casting|CastToBP_RightTread (Variables|/Script/Engine.ChildActorComponent|GetChildActor (Variables|Default|GetLeftTreadActor))))
      (Variables|Runtime|SetLeftTread _asbp_right_tread_2))))

(event EventTick
  (params (DeltaSeconds :type Float%20%28single-precision%29))
  (bind (_lefttreadspeed _righttreadspeed) (CallFunction|CalculateDifferentialDrive (Variables|Default|GetLongitudinalSpeed) (Variables|Default|GetTurnSpeed)))
  (Utilities|FlowControl|Sequence
    (:then_0
      (Default|SetSpeed (Variables|Runtime|GetLeftTread) _lefttreadspeed))
    (:then_1
      (Default|SetSpeed (Variables|Runtime|GetRightTread) _righttreadspeed))))

(fn ConstructionScript)

(fn CalculateDifferentialDrive
  (params (LongitudinalSpeed :type Float%20%28single-precision%29) (TurnSpeed :type Float%20%28single-precision%29))
  (bind _returnvalue (* TurnSpeed 0.25))
  (bind _returnvalue_2 (- LongitudinalSpeed _returnvalue))
  (bind _returnvalue_3 (+ LongitudinalSpeed _returnvalue))
  (LocalVariables|SetMaxTreadSpeed (Math|Float|Max(Float) _returnvalue_3 _returnvalue_2))
  (return _returnvalue_3 _returnvalue_2))

(fn GetCurrentSpeed
  (bind _chassis (Variables|Default|GetChassis))
  (bind _returnvalue (Physics|GetPhysicsLinearVelocity _chassis "None"))
  (return (/ (Math|Vector|DotProduct _returnvalue (Math|Transform|TransformDirection (Transformation|GetWorldTransform _chassis) "1.000000, 0, 0")) 1e+02)))