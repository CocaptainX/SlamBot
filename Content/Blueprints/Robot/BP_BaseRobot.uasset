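; Base robot Blueprint that child robots extend, linking an AI controller, odometry and LIDAR output.
; On BeginPlay it spawns its controller, passes itself to BP_BaseRobotController and calls SetupController in place of the controller's BeginPlay, then configures Odometry, optionally emulating perfect readings.
; LIDAR scans are re-broadcast through an event dispatcher.
; Setters store longitudinal and turn speeds, while GetCurrentSpeed and GetBodyMesh are stubs, the former implemented by children.
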(event `self.ReceiveBeginPlay`
  (bind _odometry (`self.Odometry`))
  (`|ExecutionSequence`
    (:`then_0`
      ;[1 1 1] Spawn the robot AI controller
      (`self.SpawnDefaultController` self)
      (bind _returnvalue (`AIBlueprintHelperLibrary.GetAIController` self))
      ;[1 1 1] Provide the AI controller with controlled robot reference
      (bind _asbp_base_robot_controller (cast `/Game/Blueprints/RobotController/BP_BaseRobotController` _returnvalue)
        (:`then`
          (set `/Game/Blueprints/RobotController/BP_BaseRobotController.ControlledRobot` self _asbp_base_robot_controller)
          ;[1 1 1] Setup the controller (use instead of BeginPlay)
          (`/Game/Blueprints/RobotController/BP_BaseRobotController.Setup Controller` _asbp_base_robot_controller))
        (:`CastFailed`
          (`KismetSystemLibrary.PrintString` "Robot AI controller does not extend BP_BaseRobotController!" true true (struct :`R` 1.0 :`A` 1.0) 30.0))))
    (:`then_1`
      ;[1 1 1] Set whether perfect odometry should be emulated and the robot reference
      (set `/Game/Blueprints/Robot/Odometry/BP_RobotOdometry.EmulatePerfectOdometry` (`self.EmulatePerfect`) _odometry)
      (set `/Game/Blueprints/Robot/Odometry/BP_RobotOdometry.Robot` self _odometry))))

(event `LidarScanComplete`
  (params (MeasurementList :type "Array of /Game/Blueprints/Robot/Lidar/ST_LidarMeasurement Structure"))
  ;[1 1 1] Call the LIDAR scan complete event dispatcher
  (`self.LidarScanEventDispatcher` MeasurementList))

(fn `GetBodyMesh`
  (returns (BodyMesh :type "StaticMeshComponent Object Reference"))
  (return null))

(fn `GetCurrentSpeed`
  (returns (CurrentSpeed :type "Float (double-precision)"))
  ;[1 1 1] This is implemented in child classes
  (return 0.0))

(fn `SetLongitudinalSpeed`
  (params (Speed :type "Float (double-precision)"))
  (set `self.LongitudinalSpeed` Speed))

(fn `SetTurnSpeed`
  (params (Speed :type "Float (double-precision)"))
  (set `self.TurnSpeed` Speed))

(fn `UserConstructionScript`)