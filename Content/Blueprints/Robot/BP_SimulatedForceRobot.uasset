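; BP_SimulatedForceRobot is a robot driven by two BP_ForceTread child actors, one on each side.
; On BeginPlay it caches both treads and attaches their Tread components to the Chassis, keeping world position.
; Each tick it applies differential drive: longitudinal plus turn speed sets the left tread, and longitudinal minus turn sets the right.
; The speed setter events defer to the parent class.
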(event `/Game/Blueprints/Robot/BP_SimulatedRobot.ReceiveBeginPlay`
  (`parent.ReceiveBeginPlay`)
  (`|ExecutionSequence`
    (:`then_0`
      (bind _asbp_force_tread (cast `/Game/Blueprints/Robot/BP_ForceTread` (`ChildActorComponent.ChildActor` (`self.ForceTreadRight`))))
      (set `self.RightTread` _asbp_force_tread)
      (`SceneComponent.K2_AttachTo` (`/Game/Blueprints/Robot/BP_ForceTread.Tread` _asbp_force_tread) (`self.Chassis`) "None" "KeepWorldPosition" true))
    (:`then_1`
      (bind _asbp_force_tread_2 (cast `/Game/Blueprints/Robot/BP_ForceTread` (`ChildActorComponent.ChildActor` (`self.ForceTreadLeft`))))
      (set `self.LeftTread` _asbp_force_tread_2)
      (`SceneComponent.K2_AttachTo` (`/Game/Blueprints/Robot/BP_ForceTread.Tread` _asbp_force_tread_2) (`self.Chassis`) "None" "KeepWorldPosition" true))))

(event `/Game/Blueprints/Robot/BP_SimulatedRobot.ReceiveTick`
  (params (DeltaSeconds :type "Float (single-precision)"))
  (bind (_lefttreadspeed _righttreadspeed) (`self.CalculateDifferentialDrive` (`self.LongitudinalSpeed`) (`self.TurnSpeed`)))
  (`|ExecutionSequence`
    (:`then_0`
      (`/Game/Blueprints/Robot/BP_ForceTread.SetSpeed` (`self.LeftTread`) _lefttreadspeed))
    (:`then_1`
      (`/Game/Blueprints/Robot/BP_ForceTread.SetSpeed` (`self.RightTread`) _righttreadspeed))))

(event `self.SetLongitudinalSpeed`
  (params (Speed :type "Float (single-precision)"))
  (`parent.SetLongitudinalSpeed` Speed))

(event `self.SetTurnSpeed`
  (params (Speed :type "Float (single-precision)"))
  (`parent.SetTurnSpeed` Speed))

(fn `CalculateDifferentialDrive`
  (params (LongitudinalSpeed :type "Float (double-precision)") (TurnSpeed :type "Float (double-precision)"))
  (returns (LeftTreadSpeed :type "Float (double-precision)") (RightTreadSpeed :type "Float (double-precision)"))
  (return (+ LongitudinalSpeed TurnSpeed) (- LongitudinalSpeed TurnSpeed)))

(fn `UserConstructionScript`)