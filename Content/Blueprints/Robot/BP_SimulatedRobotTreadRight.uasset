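; Right tread of a simulated robot, driven by physics wheels and exposing a speed setter and an average-speed readout.
; Initialize gathers tagged wheels and binds five to the parent mesh through constraints with damping-based motors.
; Each tick wakes the wheels and converts target speed to motor angular velocity using tread mesh height as diameter.
; The slowest wheel's speed drives visual wheel spin, tread material scrolling and the actual-speed debug arrow.
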(event `Initialize`
  (`|ExecutionSequence`
    (:`then_0`
      ;[1 1 1] Extract the parent static mesh component to attach to
      (bind _staticmesh (`self.GetParentStaticMesh`))
      (set `self.ParentComponent_0` _staticmesh))
    (:`then_1`
      ;[1 1 1] Setup wheels and constraints
      (`self.SetupWheels`)
      (`self.SetupConstraints` null))))

(event `self.ReceiveTick`
  (params (DeltaSeconds :type "Float (single-precision)"))
  (`|ExecutionSequence`
    (:`then_0`
      (`self.UpdateMotors`))
    (:`then_1`
      (bind _treadspeeddegreespersecond (`self.GetMinimumTreadVelocity`))
      (`self.VisualizeTreadSpeed` _treadspeeddegreespersecond DeltaSeconds))))

(fn `CalculateAngularSpeed`
  (params (SpeedMetersPerSecond :type "Float (double-precision)") (WheelDiameter :type "Float (double-precision)"))
  (returns (AngularSpeedRotationPerSecond :type "Float (double-precision)"))
  (return (/ (* SpeedMetersPerSecond 1000.0) (* WheelDiameter (`KismetMathLibrary.GetPI`)))))

(fn `ConvertDegreesPerSecondToMetersPerSecond`
  (params (DegreesPerSecond :type "Float (double-precision)"))
  (returns (MetersPerSecond :type "Float (double-precision)"))
  (bind _trackdiameter (`self.GetTrackDiameter`))
  (return (/ (* (/ DegreesPerSecond 360.0) (* _trackdiameter (`KismetMathLibrary.GetPI`))) 1000.0)))

(fn `GetAverageTreadVelocity`
  (returns (TreadSpeedDegreesPerSecond :type "Float (double-precision)"))
  (locals (SpeedSum :type "Float (double-precision)" :default 0.0))
  (for _array_element (`self.Wheels`)
    (bind _velocitydegreespersecond (`self.GetWheelSpeed` _array_element))
    (set `local.SpeedSum` (+ _velocitydegreespersecond (`local.SpeedSum`))))
  (return (/ (`local.SpeedSum`) (`KismetMathLibrary.Conv_IntToDouble` (`KismetArrayLibrary.Array_Length` (`self.Wheels`))))))

(fn `GetMinimumTreadVelocity`
  (returns (TreadSpeedDegreesPerSecond :type "Float (double-precision)"))
  (locals (MinimumSpeed :type "Float (double-precision)" :default 0.0))
  (bind _minimumspeed (`local.MinimumSpeed`))
  (for (_array_element _array_index) (`self.Wheels`)
    (bind _velocitydegreespersecond (`self.GetWheelSpeed` _array_element))
    (if (== _array_index 0)
      (set `local.MinimumSpeed` _velocitydegreespersecond :!label _label)
      (elif (< (`KismetMathLibrary.Abs` _velocitydegreespersecond) (`KismetMathLibrary.Abs` _minimumspeed))
        (goto _label))))
  (return _minimumspeed))

(fn `GetParentStaticMesh`
  (returns (StaticMesh :type "StaticMeshComponent Object Reference"))
  (bind _parents (`SceneComponent.GetParentComponents` (`self.Scene`)))
  (bind _asstatic_mesh_component (cast `StaticMeshComponent` (`KismetArrayLibrary.Array_Get` _parents (`KismetArrayLibrary.Array_LastIndex` _parents)))
    (:`then`
      _)
    (:`CastFailed`
      (`KismetSystemLibrary.PrintText` "Getting parent static mesh component failed!" true true (struct :`R` 1.0 :`A` 1.0) 30.0)))
  (return _asstatic_mesh_component))

(fn `GetTrackDiameter`
  (returns (TrackDiameter :type "Float (double-precision)"))
  (bind _returnvalue (`StaticMesh.GetBoundingBox` (`StaticMeshComponent.StaticMesh` (`self.Tread`))))
  (return (* (`KismetMathLibrary.Abs` (- (.z (`.Max` (break `Box` _returnvalue))) (.z (break `Box` _returnvalue)))) 10.0)))

(fn `GetTreadSpeed`
  (returns (SpeedMetersPerSecond :type "Float (double-precision)"))
  (bind _treadspeeddegreespersecond (`self.GetAverageTreadVelocity`))
  (bind _meterspersecond (`self.ConvertDegreesPerSecondToMetersPerSecond` _treadspeeddegreespersecond))
  (return _meterspersecond))

(fn `GetWheelSpeed`
  (params (Wheel :type "StaticMeshComponent Object Reference"))
  (returns (VelocityDegreesPerSecond :type "Float (double-precision)"))
  (bind _returnvalue (`PrimitiveComponent.GetPhysicsAngularVelocity` Wheel "None"))
  (return (* (`KismetMathLibrary.Dot_VectorVector` _returnvalue (`SceneComponent.GetForwardVector` Wheel)) -1.0)))

(fn `SetParentComponent`
  (params (Constraint :type "PhysicsConstraintComponent Object Reference") (Child :type "StaticMeshComponent Object Reference"))
  (`PhysicsConstraintComponent.SetConstrainedComponents` Constraint (`self.ParentComponent_0`) "None" Child "None"))

(fn `SetSpeed`
  (params (Speed :type "Float (double-precision)"))
  (set `self.TargetSpeed` Speed))

(fn `SetupConstraint`
  (params (Constraint :type "PhysicsConstraintComponent Object Reference") (Wheel :type "StaticMeshComponent Object Reference"))
  (`|ExecutionSequence`
    (:`then_0`
      (`PhysicsConstraintComponent.SetConstrainedComponents` Constraint (`self.ParentComponent_0`) "None" Wheel "None"))
    (:`then_1`
      (`PhysicsConstraintComponent.SetAngularDriveParams` Constraint 0.0 (`self.MotorStrength`) 0.0))
    (:`then_2`
      (`KismetArrayLibrary.Array_Add` (`self.Constraints`) Constraint))))

(fn `SetupConstraints`
  (params (Constraint :type "PhysicsConstraintComponent Object Reference") (Wheel :type "StaticMeshComponent Object Reference"))
  (`|ExecutionSequence`
    (:`then_0`
      (`self.SetupConstraint` (`self.Constraint1`) (`self.Wheel1`)))
    (:`then_1`
      (`self.SetupConstraint` (`self.Constraint2`) (`self.Wheel2`)))
    (:`then_2`
      (`self.SetupConstraint` (`self.Constraint3`) (`self.Wheel3`)))
    (:`then_3`
      (`self.SetupConstraint` (`self.Constraint4`) (`self.Wheel4`)))
    (:`then_4`
      (`self.SetupConstraint` (`self.Constraint5`) (`self.Wheel5`)))))

(fn `SetupWheel`
  (params (StaticMesh :type "StaticMeshComponent Object Reference"))
  (`KismetArrayLibrary.Array_Add` (`self.Wheels`) StaticMesh))

(fn `SetupWheels`
  (for _array_element (`self.GetComponentsByTag` "/Script/Engine.StaticMeshComponent" "Wheel")
    (bind _asstatic_mesh_component (cast `StaticMeshComponent` _array_element)
      (:`then`
        (`self.SetupWheel` _asstatic_mesh_component))
      (:`CastFailed`
        (`KismetSystemLibrary.PrintText` "Casting object to StaticMeshComponent failed!")))))

(fn `UpdateMotor`
  (params (Constraint :type "PhysicsConstraintComponent Object Reference"))
  (`self.GetTrackDiameter`)
  (bind _trackdiameter (`self.GetTrackDiameter`))
  (bind _angularspeedrotationpersecond (`self.CalculateAngularSpeed` (`self.TargetSpeed`) _trackdiameter))
  (`PhysicsConstraintComponent.SetAngularVelocityTarget` Constraint (`KismetMathLibrary.MakeVector` _angularspeedrotationpersecond)))

(fn `UpdateMotors`
  (`|ExecutionSequence`
    (:`then_0`
      (for _array_element (`self.Wheels`)
        (`PrimitiveComponent.WakeRigidBody` _array_element "None")))
    (:`then_1`
      (for _array_element_2 (`self.Constraints`)
        (`self.UpdateMotor` _array_element_2)))))

(fn `UserConstructionScript`
  (bind _returnvalue (`PrimitiveComponent.CreateDynamicMaterialInstance` (`self.Tread`) 0 null))
  (set `self.TreadMaterial` _returnvalue))

(fn `VisualizeTreadSpeed`
  (params (TreadSpeed :type "Float (double-precision)") (Delta :type "Float (double-precision)"))
  (bind _returnvalue (* TreadSpeed Delta))
  (`|ExecutionSequence`
    (:`then_0`
      (bind _meterspersecond (`self.ConvertDegreesPerSecondToMetersPerSecond` TreadSpeed))
      ;[1 1 1] Update target and actual speed arrows
      (`SceneComponent.SetRelativeScale3D` (`self.ActualSpeedArrow`) (`KismetMathLibrary.MakeVector` _meterspersecond 0.11 0.11)))
    (:`then_1`
      (`SceneComponent.SetRelativeScale3D` (`self.TargetSpeedArrow`) (`KismetMathLibrary.MakeVector` (`self.TargetSpeed`) 0.1 0.1)))
    (:`then_2`
      ;[1 1 1] Apply visual wheel rotation
      (`SceneComponent.K2_AddRelativeRotation` (`self.VisualWheelFront`) (`KismetMathLibrary.MakeRotator` _returnvalue) false false))
    (:`then_3`
      (`SceneComponent.K2_AddRelativeRotation` (`self.VisualWheelRear`) (`KismetMathLibrary.MakeRotator` _returnvalue) false false))
    (:`then_4`
      ;[1 1 1] Update tread material UV
      (bind _output_get (set `self.TreadUV` (+ (`self.TreadUV`) (* _returnvalue (`self.ThreadVisualSpeedMultiplier`)))))
      (`MaterialInstanceDynamic.SetScalarParameterValue` (`self.TreadMaterial`) "TreadOffset" _output_get))))