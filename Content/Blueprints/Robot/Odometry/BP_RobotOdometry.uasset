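; Robot odometry Blueprint that tracks position, rotation and per-step deltas for a tracked robot.
; Step selects perfect or simulated mode via EmulatePerfectOdometry.
; Simulated mode dead-reckons planar pose from tread speeds and separation using differential-drive math, scaling speeds by 100 into centimeters.
; Perfect mode reads body mesh relative transform, offsetting location from the first step; its DeltaX/Y are robot-local, whereas simulated ones follow the odometry frame.
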(fn `Step`
  (params (LeftSpeed :type "Float (double-precision)") (RightSpeed :type "Float (double-precision)") (DistanceBetweenTreads :type "Float (double-precision)"))
  (locals (LeftDistanceTravelledCentimeters :type "Float (double-precision)") (RightDistanceTravelledCentimeter :type "Float (double-precision)") (CenterDistanceTravelledCentimeter :type "Float (double-precision)") (HeadingDifferenceRadians :type "Float (double-precision)"))
  ;[1 1 1] Perform either the simulated or perfect odometry update
  (if (`self.EmulatePerfectOdometry`)
    (`self.StepPerfect`)
    (else
      (`self.StepSimulated` LeftSpeed RightSpeed DistanceBetweenTreads))))

(fn `StepPerfect`
  (locals (LeftDistanceTravelledCentimeters :type "Float (double-precision)") (RightDistanceTravelledCentimeter :type "Float (double-precision)") (CenterDistanceTravelledCentimeter :type "Float (double-precision)") (HeadingDifferenceRadians :type "Float (double-precision)"))
  (bind (_currentrotation_roll _currentrotation_pitch _currentrotation_yaw) (`KismetMathLibrary.BreakRotator` (`self.CurrentRotation`)))
  (bind (_lastrotation_roll _lastrotation_pitch _lastrotation_yaw) (`KismetMathLibrary.BreakRotator` (`self.LastRotation`)))
  (`|ExecutionSequence`
    (:`then_0`
      ;[1 1 1] Set initial location on first step
      (if (`self.IsFirstStep`)
        (set `self.IsFirstStep` false)
        (set `self.InitialLocation` (`SceneComponent.RelativeLocation` (`/Game/Blueprints/Robot/BP_BaseRobot.GetBodyMesh` (`self.Robot`))))))
    (:`then_1`
      ;[1 1 1] Set last and current positition
      (set `self.LastPosition` (`self.CurrentPosition`)))
    (:`then_2`
      (set `self.CurrentPosition` (- (`SceneComponent.RelativeLocation` (`/Game/Blueprints/Robot/BP_BaseRobot.GetBodyMesh` (`self.Robot`))) (`self.InitialLocation`))))
    (:`then_3`
      ;[1 1 1] Set last and current rotation
      (set `self.LastRotation` (`self.CurrentRotation`)))
    (:`then_4`
      (set `self.CurrentRotation` (`SceneComponent.RelativeRotation` (`/Game/Blueprints/Robot/BP_BaseRobot.GetBodyMesh` (`self.Robot`)))))
    (:`then_5`
      ;[1 1 1] Update delta position and yaw
      (bind _output_get (set `self.DeltaPosition` (- (`self.CurrentPosition`) (`self.LastPosition`))))
      (set `self.DeltaYaw` (- _currentrotation_yaw _lastrotation_yaw)))
    (:`then_6`
      (bind (_returnvalue_x _returnvalue_y) (`KismetMathLibrary.BreakVector` (`KismetMathLibrary.LessLess_VectorRotator` _output_get (`self.K2_GetComponentRotation` (`/Game/Blueprints/Robot/BP_BaseRobot.GetBodyMesh` (`self.Robot`))))))
      ;[1 1 1] Update delta X and Y in local robot coordinates
      (set `self.DeltaX` _returnvalue_x)
      (set `self.DeltaY` _returnvalue_y))))

(fn `StepSimulated`
  (params (LeftSpeed :type "Float (double-precision)") (RightSpeed :type "Float (double-precision)") (DistanceBetweenTreads :type "Float (double-precision)"))
  (locals (LeftDistanceTravelledCentimeters :type "Float (double-precision)") (RightDistanceTravelledCentimeter :type "Float (double-precision)") (CenterDistanceTravelledCentimeter :type "Float (double-precision)") (HeadingDifferenceRadians :type "Float (double-precision)"))
  (bind (_currentposition_x _currentposition_y) (`KismetMathLibrary.BreakVector` (`self.CurrentPosition`)))
  (bind (_currentrotation_roll _currentrotation_pitch _currentrotation_yaw) (`KismetMathLibrary.BreakRotator` (`self.CurrentRotation`)))
  (bind (_currentrotation_roll_2 _currentrotation_pitch_2 _currentrotation_yaw_2) (`KismetMathLibrary.BreakRotator` (`self.CurrentRotation`)))
  (bind (_currentrotation_roll_3 _currentrotation_pitch_3 _currentrotation_yaw_3) (`KismetMathLibrary.BreakRotator` (`self.CurrentRotation`)))
  (bind (_currentrotation_roll_4 _currentrotation_pitch_4 _currentrotation_yaw_4) (`KismetMathLibrary.BreakRotator` (`self.CurrentRotation`)))
  (bind (_lastrotation_roll _lastrotation_pitch _lastrotation_yaw) (`KismetMathLibrary.BreakRotator` (`self.LastRotation`)))
  (bind _returnvalue (* (`local.CenterDistanceTravelledCentimeter`) (`KismetMathLibrary.DegSin` _currentrotation_yaw_2)))
  (bind _returnvalue_2 (* (`local.CenterDistanceTravelledCentimeter`) (`KismetMathLibrary.DegCos` _currentrotation_yaw_3)))
  (`|ExecutionSequence`
    (:`then_0`
      ;[1 1 1] Calculate left, right and center distances travelled
      (set `local.LeftDistanceTravelledCentimeters` (* (* LeftSpeed (`GameplayStatics.GetWorldDeltaSeconds`)) 100.0)))
    (:`then_1`
      (set `local.RightDistanceTravelledCentimeter` (* (* RightSpeed (`GameplayStatics.GetWorldDeltaSeconds`)) 100.0)))
    (:`then_2`
      (set `local.CenterDistanceTravelledCentimeter` (/ (+ (`local.LeftDistanceTravelledCentimeters`) (`local.RightDistanceTravelledCentimeter`)) 2.0)))
    (:`then_3`
      ;[1 1 1] Calculate heading change
      (set `local.HeadingDifferenceRadians` (/ (- (`local.LeftDistanceTravelledCentimeters`) (`local.RightDistanceTravelledCentimeter`)) DistanceBetweenTreads)))
    (:`then_4`
      ;[1 1 1] Update last position and rotation
      (set `self.LastPosition` (`self.CurrentPosition`))
      (set `self.LastRotation` (`self.CurrentRotation`)))
    (:`then_5`
      ;[1 1 1] Calculate new position
      (set `self.CurrentPosition` (`KismetMathLibrary.MakeVector` (+ _currentposition_x _returnvalue_2) (+ _currentposition_y _returnvalue)))
      ;[1 1 1] Update delta position
      (set `self.DeltaX` _returnvalue_2)
      (set `self.DeltaY` _returnvalue))
    (:`then_6`
      ;[1 1 1] Calculate new rotation
      (set `self.CurrentRotation` (`KismetMathLibrary.MakeRotator` 0.0 0.0 (+ _currentrotation_yaw (`KismetMathLibrary.RadiansToDegrees` (`local.HeadingDifferenceRadians`))))))
    (:`then_7`
      ;[1 1 1] Update deltas
      (set `self.DeltaPosition` (- (`self.CurrentPosition`) (`self.LastPosition`)))
      (set `self.DeltaYaw` (- _currentrotation_yaw_4 _lastrotation_yaw)))))