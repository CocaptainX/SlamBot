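; BP_ManualRobotController lets the player drive a controlled robot manually.
; On BeginPlay it enables input from player controller 0 and creates a UI_ManualControllerWidget, handing it a reference to itself.
; Speed and Turn axis inputs are scaled by maximum linear and angular rates and sent to the robot as longitudinal and turn speeds.
; A TogglePause action pauses and unpauses the game.
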(event `self.ReceiveBeginPlay`
  ;[1 1 1] Setup manual controller
  (`parent.ReceiveBeginPlay`)
  (`self.CreateControllerWidget`)
  (`self.EnableInput` (`GameplayStatics.GetPlayerController` 0))
  (`KismetSystemLibrary.PrintString` "Created manual robot controller"))

(event `InputAxis|Speed`
  (params (AxisValue :type "Float (single-precision)"))
  ;[1 1 1] Set robot longitudinal speed
  (bind _output_get (set `self.SpeedRate` AxisValue))
  (`/Game/Blueprints/Robot/BP_BaseRobot.SetLongitudinalSpeed` (`self.ControlledRobot`) (* _output_get (`self.MaxSpeed`))))

(event `InputAxis|Turn`
  (params (AxisValue :type "Float (single-precision)"))
  ;[1 1 1] Set robot turn speed
  (bind _output_get (set `self.TurnRate` AxisValue))
  (`/Game/Blueprints/Robot/BP_BaseRobot.SetTurnSpeed` (`self.ControlledRobot`) (* _output_get (`self.MaxTurnOmega`))))

(event `InputAction|TogglePause` :paused true
  (params (Key :type "Key Structure" :default "AnyKey"))
  ;[1 1 1] Toggle pause
  (:`Pressed`
    (if (`GameplayStatics.IsGamePaused`)
      (`GameplayStatics.SetGamePaused` false)
      (`KismetSystemLibrary.PrintString` "Unpaused")
      (else
        (`GameplayStatics.SetGamePaused` true)
        (`KismetSystemLibrary.PrintString` "Paused"))))
  (:`Released`
    (`KismetSystemLibrary.PrintString` "Pause released")))

(fn `CreateControllerWidget`
  (bind _returnvalue (`|CreateWidget` "/Game/UI/UI_ManualControllerWidget.UI_ManualControllerWidget_C"))
  (bind _output_get (set `self.ManulControllerWidget` _returnvalue))
  (`UserWidget.AddToViewport` _output_get 0)
  (set `/Game/UI/UI_ManualControllerWidget.ManualPlayerController` self _output_get))

(fn `UserConstructionScript`)