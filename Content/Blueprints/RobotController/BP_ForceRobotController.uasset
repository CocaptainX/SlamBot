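; Robot controller that steers a robot by force-field navigation, with a UI widget and toggles for manual driving and LIDAR.
; LIDAR hits become force fields on a spawned BP_ForceNavigator, cleared per scan and shifted by odometry each update.
; The combined push force's angle sets turn speed, and forward speed drops as turning increases.
; An initial force wall spawns behind the robot; periodic wall renewal and purging are disconnected.
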(event `self.ReceiveBeginPlay`
  (`parent.ReceiveBeginPlay`)
  (`|ExecutionSequence`
    (:`then_0`
      ;[1 1 1] Request input, used for manual control (toggle with ENTER)
      (`self.EnableInput` (`GameplayStatics.GetPlayerController` 0)))
    (:`then_1`
      ;[1 1 1] Create force controller UI widget
      (bind _returnvalue (`|CreateWidget` "/Game/UI/UI_ForceControllerWidget.UI_ForceControllerWidget_C" null self))
      (`UserWidget.AddToViewport` _returnvalue 0))))

(event `self.Initialize`
  (params (Robot :type "/Game/Blueprints/Robot/BP_BaseRobot Object Reference"))
  (bind _robot (`self.Robot`))
  (bind _robot_2 (`self.Robot`))
  (`parent.Initialize` Robot)
  (`|ExecutionSequence`
    (:`then_0`
      ;[1 1 1] Bind to robot LIDAR events
      (add `/Game/Blueprints/Robot/BP_BaseRobot.OnLidarMeasurement` _robot (delegate `OnLidarMeasurement`))
      (add `/Game/Blueprints/Robot/BP_BaseRobot.OnLidarScan` _robot (delegate `OnLidarScan`)))
    (:`then_1`
      ;[1 1 1] Create the force navigator
      (bind _returnvalue (`|SpawnActorFromClass` "/Game/Blueprints/ForceNavigator/BP_ForceNavigator.BP_ForceNavigator_C" (`self.GetTransform` _robot_2) "Undefined" "OverrideRootScale" _robot_2 (`/Game/Blueprints/Robot/BP_BaseRobot.Debug` _robot_2) true))
      (bind _output_get (set `self.ForceNavigator` _returnvalue))
      (`SceneComponent.K2_AttachToComponent` (`self.K2_GetRootComponent` _output_get) (`/Game/Blueprints/Robot/BP_BaseRobot.GetBodyMesh` (`self.Robot`)) "None" "KeepWorld" "KeepWorld" "KeepWorld" true)
      (`/Game/Blueprints/ForceNavigator/BP_ForceNavigator.Initialize` _output_get true))
    (:`then_2`
      ;[1 1 1] Create the first force wall behind the robot
      (`self.CreateOdometryForceWall`))))

(event `self.Update`
  (params (DeltaSeconds :type "Float (single-precision)"))
  (bind _robot (`self.Robot`))
  (bind (_deltalastodometryforcelocation_x _deltalastodometryforcelocation_y) (`KismetMathLibrary.BreakVector` (`self.DeltaLastOdometryForceLocation`)))
  (bind _robot_2 (`self.Robot`))
  (bind _odometry (`/Game/Blueprints/Robot/BP_BaseRobot.Odometry` _robot))
  (bind _odometry_2 (`/Game/Blueprints/Robot/BP_BaseRobot.Odometry` (`self.Robot`)))
  (`|ExecutionSequence`
    (:`then_0`
      ;[1 1 1] Move force fields by odometry step
      (`/Game/Blueprints/ForceNavigator/BP_ForceNavigator.ApplyOdometry` (`self.ForceNavigator`) (`KismetMathLibrary.MakeVector` (`/Game/Blueprints/Robot/Odometry/BP_RobotOdometry.DeltaX` _odometry) (`/Game/Blueprints/Robot/Odometry/BP_RobotOdometry.DeltaY` _odometry)) (`/Game/Blueprints/Robot/Odometry/BP_RobotOdometry.DeltaYaw` _odometry) (`SceneComponent.GetUpVector` (`/Game/Blueprints/Robot/BP_BaseRobot.GetBodyMesh` _robot))))
    (:`then_1`
      ;[1 1 1] Move the last odometry force location by odometry
      (set `self.DeltaLastOdometryForceLocation` (`KismetMathLibrary.RotateAngleAxis` (`KismetMathLibrary.MakeVector` (- _deltalastodometryforcelocation_x (`/Game/Blueprints/Robot/Odometry/BP_RobotOdometry.DeltaX` _odometry_2)) (- _deltalastodometryforcelocation_y (`/Game/Blueprints/Robot/Odometry/BP_RobotOdometry.DeltaY` _odometry_2))) (`/Game/Blueprints/Robot/Odometry/BP_RobotOdometry.DeltaYaw` _odometry_2) (0.0 0.0 1.0))))
    (:`then_2`
      ;[1 1 1] Add odometry-based force field behind the robot at set distances apart
      (if (>= (`KismetMathLibrary.VSize` (`self.DeltaLastOdometryForceLocation`)) (`self.OdometryForceWallDistanceInterval`))
        _))
    (:`then_3`
      ;[1 1 1] Calculate robot longitudinal and turn speed based on combined push force and apply it
      (bind _pushforceangle (`self.CalculatePushForceAngle` (`/Game/Blueprints/ForceNavigator/BP_ForceNavigator.PushForce` (`self.ForceNavigator`))))
      (bind _output_get (set `self.PushForceAngle` _pushforceangle))
      (if (not (`self.UseManualControl`))
        (bind (_longitudinalspeed _turnspeed) (`self.CalculateRobotSpeed` _output_get))
        (`/Game/Blueprints/Robot/BP_BaseRobot.SetLongitudinalSpeed` _robot_2 _longitudinalspeed)
        (`/Game/Blueprints/Robot/BP_BaseRobot.SetTurnSpeed` _robot_2 _turnspeed)))))

(event `OnLidarMeasurement`
  (params (Measurement :type "/Game/Blueprints/Robot/Lidar/ST_LidarMeasurement Structure"))
  (bind (_index _distance _angle _signalstrength) (break `/Game/Blueprints/Robot/Lidar/ST_LidarMeasurement` Measurement))
  ;[1 1 1] Only continue if LIDAR is active
  (if (`self.IsLidarActive`)
    ;[1 1 1] Convert to cartesian coordinates
    (bind _location (`/Game/Blueprints/FunctionLibraries/Math.PolarToCartesian` _distance _angle))
    ;[1 1 1] Create the force field
    (`/Game/Blueprints/ForceNavigator/BP_ForceNavigator.CreateForceField` (`self.ForceNavigator`) _location (* (`KismetMathLibrary.Conv_IntToDouble` _signalstrength) (`self.SignalStrengthToMagnitudeMultiplier`)) (`self.INFINITE_LIFETIME`) (`self.LidarScanCount`))))

(event `OnLidarScan`
  (params (MeasurementList :type "Array of /Game/Blueprints/Robot/Lidar/ST_LidarMeasurement Structure (by ref)"))
  (bind _forcenavigator (`self.ForceNavigator`))
  ;[1 1 1] Only continue if LIDAR is active
  (if (`self.IsLidarActive`)
    ;[1 1 1] Clear LIDAR forcefields from last scan
    (`/Game/Blueprints/ForceNavigator/BP_ForceNavigator.ClearByGroupId` (`self.ForceNavigator`) (- (`self.LidarScanCount`) 1))
    ;[1 1 1] Increment scan count
    (set `self.LidarScanCount` (+ (`self.LidarScanCount`) 1))
    (`KismetSystemLibrary.PrintText` (`|FormatText` "real: {count}, visual: {visual}" (`KismetArrayLibrary.Array_Length` (`/Game/Blueprints/ForceNavigator/BP_ForceNavigator.ForceFields` _forcenavigator)) (`KismetArrayLibrary.Array_Length` (`/Game/Blueprints/ForceNavigator/BP_ForceNavigator.ForceFieldVisuals` _forcenavigator))))))

(event `InputAxis|Speed`
  (params (AxisValue :type "Float (single-precision)"))
  ;[1 1 1] Set robot longitudinal speed
  (if (`self.UseManualControl`)
    (bind _output_get (set `self.SpeedRate` AxisValue))
    (`/Game/Blueprints/Robot/BP_BaseRobot.SetLongitudinalSpeed` (`self.Robot`) (* _output_get (`self.MaxLongitudinalSpeed`)))))

(event `InputAxis|Turn`
  (params (AxisValue :type "Float (single-precision)"))
  ;[1 1 1] Set robot turn speed
  (if (`self.UseManualControl`)
    (bind _output_get (set `self.TurnRate` AxisValue))
    (`/Game/Blueprints/Robot/BP_BaseRobot.SetTurnSpeed` (`self.Robot`) (* _output_get (`self.MaxTurnSpeed`)))))

(event `InputAction|ToggleMode`
  (params (Key :type "Key Structure" :default "AnyKey"))
  (:`Pressed`
    ;[1 1 1] Toggle manual control over the robot
    (if (`self.UseManualControl`)
      (set `self.UseManualControl` false)
      (`KismetSystemLibrary.PrintText` "Now using manual control")
      (else
        (set `self.UseManualControl` true)
        (`KismetSystemLibrary.PrintText` "Now using automatic control")))))

(event `InputAction|ToggleLidar`
  (params (Key :type "Key Structure" :default "AnyKey"))
  (:`Pressed`
    ;[1 1 1] Toggle whether LIDAR is active
    (if (`self.IsLidarActive`)
      (set `self.IsLidarActive` false)
      (`KismetSystemLibrary.PrintText` "Deactivated LIDAR")
      (else
        (set `self.IsLidarActive` true)
        (`KismetSystemLibrary.PrintText` "Activated LIDAR")))))

(fn `CalculateForceFieldLocation`
  (params (Angle :type "Float (double-precision)") (Distance :type "Float (double-precision)"))
  (returns (Location :type "Vector Structure"))
  (return (* (`KismetMathLibrary.GreaterGreater_VectorRotator` (`KismetMathLibrary.MakeVector` 1.0) (`KismetMathLibrary.MakeRotator` 0.0 0.0 Angle)) Distance)))

(fn `CalculateLongitudinalSpeed`
  (params (TurnSpeed :type "Float (double-precision)"))
  (returns (LongitudinalSpeed :type "Float (double-precision)"))
  (return (- (`self.MaxLongitudinalSpeed`) (* (/ (`KismetMathLibrary.Abs` TurnSpeed) (`self.MaxTurnSpeed`)) (`self.MaxLongitudinalSpeed`)))))

(fn `CalculatePushForceAngle`
  (params (PushForce :type "Vector Structure"))
  (returns (PushForceAngle :type "Float (double-precision)"))
  (bind (_returnvalue_roll _returnvalue_pitch _returnvalue_yaw) (`KismetMathLibrary.BreakRotator` (`KismetMathLibrary.MakeRotationFromAxes` PushForce (0.0 1.0 0.0) (0.0 0.0 1.0))))
  (return _returnvalue_yaw))

(fn `CalculateRobotSpeed`
  (params (PushForceAngle :type "Float (double-precision)"))
  (returns (LongitudinalSpeed :type "Float (double-precision)") (TurnSpeed :type "Float (double-precision)"))
  (locals (Angle :type "Float (double-precision)"))
  (bind _turnspeed (`self.CalculateTurnSpeed` PushForceAngle (`self.MaxTurnSpeed`)))
  (bind _longitudinalspeed (`self.CalculateLongitudinalSpeed` _turnspeed))
  (return _longitudinalspeed _turnspeed))

(fn `CalculateTurnSpeed`
  (params (SignedPushAngleDegrees :type "Float (double-precision)") (MaxTurnSpeed :type "Float (double-precision)"))
  (returns (TurnSpeed :type "Float (double-precision)"))
  (return (`KismetMathLibrary.FClamp` (* (/ SignedPushAngleDegrees 90.0) (`self.MaxTurnSpeed`)) (* MaxTurnSpeed -1.0) MaxTurnSpeed)))

(fn `CreateOdometryForceWall`
  (bind _odometryforcewallfieldcount (`self.OdometryForceWallFieldCount`))
  (for _index (range _odometryforcewallfieldcount)
    (bind _createdforcefieldid (`/Game/Blueprints/ForceNavigator/BP_ForceNavigator.CreateForceField` (`self.ForceNavigator`) (`KismetMathLibrary.MakeVector` (* (`self.OdometryForceWallDistanceInterval`) -1.0) (* (- _index (/ _odometryforcewallfieldcount 2)) (`self.OdometryForceWallDistanceStep`))) (`self.OdometryForceFieldMagnitude`) (`self.INFINITE_LIFETIME`) (`self.FORCE_FIELD_GROUP_ODOMETRY`)))
    (`KismetArrayLibrary.Array_Add` (`self.OdometryForceFieldIds`) _createdforcefieldid)))

(fn `GetSignedAngleBetweenVectors`
  (params (A :type "Vector Structure") (B :type "Vector Structure") (Normal :type "Vector Structure"))
  (returns (SignedAngleDegrees :type "Float (double-precision)"))
  (bind _returnvalue (`KismetMathLibrary.DegAcos` (`KismetMathLibrary.Dot_VectorVector` (`KismetMathLibrary.Normal` A) (`KismetMathLibrary.Normal` B))))
  ;[1 1 1] Calculate whether the angle is negative or positive
  (if (< (`KismetMathLibrary.Dot_VectorVector` Normal (`KismetMathLibrary.Cross_VectorVector` A B)) 0.0)
    ;[1 1 1] Calculate and return signed angle
    (return (* _returnvalue -1.0))
    (else
      (return _returnvalue))))

(fn `PurgeOdometryForceFields`
  (bind _odometryforcefieldids (`self.OdometryForceFieldIds`))
  (while (> (`KismetArrayLibrary.Array_Length` _odometryforcefieldids) (`self.MaxOdometryForceFieldCount`))
    (`/Game/Blueprints/ForceNavigator/BP_ForceNavigator.RemoveForceFieldById` (`self.ForceNavigator`) (`KismetArrayLibrary.Array_Get` _odometryforcefieldids))
    (`KismetArrayLibrary.Array_Remove` _odometryforcefieldids)))

(fn `UserConstructionScript`)