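; Player controller for manually driving the game mode's robot.
; On BeginPlay it creates the UI_ManualController widget, adds it to the viewport and hands it a reference to itself.
; The Speed axis, scaled by MaxSpeed, goes every update to SetSpeed on the Robot found through a cast to BP_BaseGameMode.
; The ToggleMouse action shows or hides the mouse cursor.
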(event `self.ReceiveBeginPlay`
  (`self.CreateControllerWidget`))

(event `InputAction|ToggleMouse`
  (params (Key :type "Key Structure" :default "AnyKey"))
  (:`Pressed`
    (`KismetSystemLibrary.PrintText` "Toggle mouse")
    (if (`self.bShowMouseCursor`)
      (set `self.bShowMouseCursor` false)
      (else
        (set `self.bShowMouseCursor` true)))))

(event `InputAxis|Speed`
  (params (AxisValue :type "Float (single-precision)"))
  (bind _output_get (set `self.SpeedRate` AxisValue))
  (bind _activegamemode (`self.GetActiveGameMode`))
  (`/Game/Blueprints/BP_BaseRobot.SetSpeed` (`/Game/Blueprints/BP_BaseGameMode.Robot` _activegamemode) (* _output_get (`self.MaxSpeed`))))

(fn `CreateControllerWidget`
  (bind _returnvalue (`|CreateWidget` "/Game/UI/UI_ManualController.UI_ManualController_C"))
  (bind _output_get (set `self.ManulControllerWidget` _returnvalue))
  (`UserWidget.AddToViewport` _output_get 0)
  (set `/Game/UI/UI_ManualController.ManualPlayerController` self _output_get))

(fn `GetActiveGameMode`
  (returns (ActiveGameMode :type "/Game/Blueprints/BP_BaseGameMode Object Reference"))
  (bind _asbp_base_game_mode (cast `/Game/Blueprints/BP_BaseGameMode` (`GameplayStatics.GetGameMode`))
    (:`then`
      _)
    (:`CastFailed`
      (`KismetSystemLibrary.PrintText` "Getting active base game mode failed!" true true (struct :`R` 1.0 :`A` 1.0) 30.0)))
  (return _asbp_base_game_mode))

(fn `UserConstructionScript`)