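; BP_SerialDebugger is a test actor that opens a serial port and shows its name, connection status or error, and queued message count on text components.
; Each tick it refreshes the readouts, then drains the incoming message queue by printing every message.
; Actor overlap begin and end send LED on/off commands over the port and recolor the status text, with the LED also switched off at begin and end of play.
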(event `self.ReceiveBeginPlay`
  (`self.UpdateSerialPortNameText`)
  (`self.OpenSerialPort`)
  (`self.SetLedState` false))

(event `self.ReceiveEndPlay`
  (params (EndPlayReason :type "EEndPlayReason Enum" :default "Destroyed"))
  (`self.SetLedState` false))

(event `self.ReceiveTick`
  (params (DeltaSeconds :type "Float (single-precision)"))
  (`self.UpdateMessageCountText`)
  (`self.UpdateStatusText`)
  (`self.LogQueuedMessages`))

(event `self.ReceiveActorBeginOverlap`
  (params (OtherActor :type "Actor Object Reference"))
  (`self.SetLedState` true))

(event `self.ReceiveActorEndOverlap`
  (params (OtherActor :type "Actor Object Reference"))
  (`self.SetLedState` false))

(fn `LogQueuedMessages`
  (while (> (`self.MessageCount`) 0)
    (bind _returnvalue (`self.GetNextMessage`))
    (`KismetSystemLibrary.PrintText` (`|FormatText` "Got message: {message}" (`KismetTextLibrary.Conv_StringToText` _returnvalue)))))

(fn `OpenSerialPort`
  (`self.OpenPort` (`self.SerialPortName`)))

(fn `SetLedState`
  (params (IsOn :type Boolean))
  (if IsOn
    (`self.SendMessage` "<led:on>")
    (`TextRenderComponent.SetTextRenderColor` (`self.StatusText`) (make `Color` 0 0 255))
    (else
      (`self.SendMessage` "<led:off>")
      (`TextRenderComponent.SetTextRenderColor` (`self.StatusText`) (make `Color` 0)))))

(fn `UpdateMessageCountText`
  (`TextRenderComponent.K2_SetText` (`self.MessageCountText`) (`|FormatText` "Queued message count: {count}" (`KismetTextLibrary.Conv_IntToText` (`self.MessageCount`)))))

(fn `UpdateSerialPortNameText`
  (`TextRenderComponent.K2_SetText` (`self.SerialPortNameText`) (`|FormatText` "Port: {name}" (`KismetTextLibrary.Conv_StringToText` (`self.SerialPortName`)))))

(fn `UpdateStatusText`
  (if (`self.IsConnected`)
    (set `self.StatusName` "Connected")
    (else
      (set `self.StatusName` (`self.ErrorMessage`))))
  (`TextRenderComponent.K2_SetText` (`self.StatusText`) (`KismetTextLibrary.Conv_StringToText` (`self.StatusName`))))

(fn `UserConstructionScript`)