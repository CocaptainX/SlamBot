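; BP_BaseRobotController is a base robot controller that provides lookup helpers and has no active event logic.
; GetActiveGameMode returns the current game mode cast to BP_BaseGameMode.
; GetControlledRobot returns the controlled pawn as BP_Robot_Base.
; If that cast fails, it scans all robot actors and returns the first without a valid AI controller.
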(fn `GetActiveGameMode`
  (returns (ActiveGameMode :type "/Game/Blueprints/GameMode/BP_BaseGameMode Object Reference"))
  (bind _asbp_base_game_mode (cast `/Game/Blueprints/GameMode/BP_BaseGameMode` (`GameplayStatics.GetGameMode`))
    (:`then`
      _)
    (:`CastFailed`
      _))
  (return _asbp_base_game_mode))

(fn `GetControlledRobot`
  (returns (ControlledRobot :type "/Game/Blueprints/Robot/BP_Robot_Base Object Reference"))
  ;[1 1 1] Use controlled pawn if available
  (bind _asbp_robot_base (cast `/Game/Blueprints/Robot/BP_Robot_Base` (`self.K2_GetPawn`))
    (:`then`
      (return _asbp_robot_base))
    (:`CastFailed`
      ;[1 1 1] Find base robot without AI controller
      (bind _outactors (`GameplayStatics.GetAllActorsOfClass` "/Game/Blueprints/Robot/BP_Robot_Base.BP_Robot_Base_C"))
      (for _array_element _outactors
        (bind _returnvalue (`AIBlueprintHelperLibrary.GetAIController` _array_element))
        (if (not (`KismetSystemLibrary.IsValid` _returnvalue))
          (return _array_element))))))

(fn `UserConstructionScript`)