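; BP_ManualPlayerController is a player controller for manually driving the active game mode's robot.
; Speed and Turn axis inputs are scaled by maximum speed and turn rate, then sent to the robot as longitudinal and turn speeds.
; On BeginPlay it adds a manual controller widget to the viewport and hands it a reference to itself.
; A ToggleMouse action shows or hides the cursor.
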(event `self.ReceiveBeginPlay`
  ;[1 1 1] Setup manual controller
  (`self.CreateControllerWidget`))

(event `InputAction|ToggleMouse`
  (params (Key :type "Key Structure" :default "AnyKey"))
  ;[1 1 1] Toggle mouse cursor visibility
  (:`Pressed`
    (`KismetSystemLibrary.PrintText` "Toggle mouse")
    (if (`self.bShowMouseCursor`)
      (set `self.bShowMouseCursor` false)
      (else
        (set `self.bShowMouseCursor` true)))))

(event `InputAxis|Speed`
  (params (AxisValue :type "Float (single-precision)"))
  ;[1 1 1] Set robot longitudinal speed
  (bind _output_get (set `self.SpeedRate` AxisValue))
  (bind _activegamemode (`self.GetActiveGameMode`))
  (`/Game/Blueprints/Robot/BP_BaseRobot.SetLongitudinalSpeed` (`/Game/Blueprints/GameMode/BP_BaseGameMode.Robot` _activegamemode) (* _output_get (`self.MaxSpeed`))))

(event `InputAxis|Turn`
  (params (AxisValue :type "Float (single-precision)"))
  ;[1 1 1] Set robot turn speed
  (bind _output_get (set `self.TurnRate` AxisValue))
  (bind _activegamemode (`self.GetActiveGameMode`))
  (`/Game/Blueprints/Robot/BP_BaseRobot.SetTurnSpeed` (`/Game/Blueprints/GameMode/BP_BaseGameMode.Robot` _activegamemode) (* _output_get (`self.MaxTurnOmega`))))

(fn `CreateControllerWidget`
  (bind _returnvalue (`|CreateWidget` "/Game/UI/UI_ManualControllerWidget.UI_ManualControllerWidget_C"))
  (bind _output_get (set `self.ManulControllerWidget` _returnvalue))
  (`UserWidget.AddToViewport` _output_get 0)
  (set `/Game/UI/UI_ManualControllerWidget.ManualPlayerController` self _output_get))

(fn `UserConstructionScript`)