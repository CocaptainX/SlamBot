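; Player controller for manually driving a robot, with a toggle between possessing the robot and the first BP_Pawn in the level.
; Speed and turn axis inputs are scaled by maximum rates and sent to the controlled robot as longitudinal and turn speeds.
; On BeginPlay it creates the manual controller widget and gives it a self-reference.
; Another input toggles the mouse cursor.
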(event `self.ReceiveBeginPlay`
  ;[1 1 1] Setup manual controller
  (`parent.ReceiveBeginPlay`)
  (`self.CreateControllerWidget`))

(event `InputAction|ToggleMouse`
  (params (Key :type "Key Structure" :default "AnyKey"))
  ;[1 1 1] Toggle mouse cursor visibility
  (:`Pressed`
    (`KismetSystemLibrary.PrintText` "Toggle mouse")
    (if (`self.bShowMouseCursor`)
      (set `self.bShowMouseCursor` false)
      (else
        (set `self.bShowMouseCursor` true)))))

(event `InputAction|TogglePossess`
  (params (Key :type "Key Structure" :default "AnyKey"))
  ;[1 1 1] Toggle posessing the robot
  (:`Pressed`
    (cast `/Game/Blueprints/Robot/BP_BaseRobot` (`self.K2_GetPawn`)
      (:`then`
        (`self.GetControlledRobot`)
        (bind _outactors (`GameplayStatics.GetAllActorsOfClass` "/Game/Blueprints/Pawn/BP_Pawn.BP_Pawn_C"))
        (`self.Possess` (`KismetArrayLibrary.Array_Get` _outactors)))
      (:`CastFailed`
        (bind _controlledrobot (`self.GetControlledRobot`))
        (`self.Possess` _controlledrobot)))))

(event `InputAxis|Speed`
  (params (AxisValue :type "Float (single-precision)"))
  ;[1 1 1] Set robot longitudinal speed
  (bind _output_get (set `self.SpeedRate` AxisValue))
  (bind _controlledrobot (`self.GetControlledRobot`))
  (`/Game/Blueprints/Robot/BP_BaseRobot.SetLongitudinalSpeed` _controlledrobot (* _output_get (`self.MaxSpeed`))))

(event `InputAxis|Turn`
  (params (AxisValue :type "Float (single-precision)"))
  ;[1 1 1] Set robot turn speed
  (bind _output_get (set `self.TurnRate` AxisValue))
  (bind _controlledrobot (`self.GetControlledRobot`))
  (`/Game/Blueprints/Robot/BP_BaseRobot.SetTurnSpeed` _controlledrobot (* _output_get (`self.MaxTurnOmega`))))

(event `InputAxis|LeftAxisX`
  (params (AxisValue :type "Float (single-precision)")))

(event `InputAxis|RightAxisY`
  (params (AxisValue :type "Float (single-precision)")))

(fn `CreateControllerWidget`
  (bind _returnvalue (`|CreateWidget` "/Game/UI/UI_ManualControllerWidget.UI_ManualControllerWidget_C"))
  (bind _output_get (set `self.ManulControllerWidget` _returnvalue))
  (`UserWidget.AddToViewport` _output_get 0)
  (set `/Game/UI/UI_ManualControllerWidget.ManualPlayerController` self _output_get))

(fn `UserConstructionScript`)