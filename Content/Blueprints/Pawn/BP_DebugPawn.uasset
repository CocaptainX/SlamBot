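; Debug fly-camera pawn that moves around the world and drags physics objects with the mouse.
; Input flags drive local-space forces on Tick, with a fast multiplier, while angular velocity is zeroed and mouse axes set yaw and clamped pitch.
; Showing the cursor disables panning and allows picking: a camera trace grabs simulating components through a PhysicsHandle at fixed distance, with Left Alt selecting hit-point grabs with free rotation.
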(event EventTick
  (params (DeltaSeconds :type Float%20%28single-precision%29))
  (Utilities|FlowControl|Sequence
    (:then_0
      ;[1 1 1] Move camera
      (if (Variables|Movement|GetIsMovementEnabled)
        (Utilities|FlowControl|Sequence
          (:then_0
            (if (Variables|Movement|GetIsMovingForward)
              (CallFunction|MovePawn "1.000000, 0, 0" (Variables|Config|GetMovementSpeed))))
          (:then_1
            (if (Variables|Movement|GetIsMovingBackward)
              (CallFunction|MovePawn "-1.000000, 0, 0" (Variables|Config|GetMovementSpeed))))
          (:then_2
            (if (Variables|Movement|GetIsMovingRight)
              (CallFunction|MovePawn "0.000000,1.000000,0.000000" (Variables|Config|GetMovementSpeed))))
          (:then_3
            (if (Variables|Movement|GetIsMovingLeft)
              (CallFunction|MovePawn "0.000000,-1.000000,0.000000" (Variables|Config|GetMovementSpeed)))))))
    (:then_1
      ;[1 1 1] Clear angular velocity
      (Class|PrimitiveComponent|SetPhysicsAngularVelocity (Variables|Default|GetPawn) "0, 0, 0" false "None"))
    (:then_2
      (CallFunction|ApplyPickerForces))))

(event Input|ActionEvents|InputActionMoveFast
  (params (Key :type Key%20Structure :default "AnyKey"))
  ;[1 1 1] Capture special movement
  (:Pressed
    (Variables|Movement|SetIsMovingFast true))
  (:Released
    (Variables|Movement|SetIsMovingFast false)))

(event Input|ActionEvents|InputActionPickObject
  (params (Key :type Key%20Structure :default "AnyKey"))
  ;[1 1 1] Enable and disable picker
  (:Pressed
    (if (and (Variables|/Script/Engine.PlayerController|GetbShowMouseCursor (Game|GetPlayerController 0)) (not (Variables|Picker|GetIsPickerEnabled)))
      (CallFunction|EnablePicker)))
  (:Released
    (if (Variables|Picker|GetIsPickerEnabled)
      (CallFunction|DisablePicker))))

(event Input|ActionEvents|InputActionShowMouse
  (params (Key :type Key%20Structure :default "AnyKey"))
  ;[1 1 1] Show mouse cursor when ctrl is pressed
  (:Pressed
    (CallFunction|ShowMouseCursor))
  (:Released
    (CallFunction|HideMouseCursor)))

(event Input|ActionEvents|InputActionMoveForward
  (params (Key :type Key%20Structure :default "AnyKey"))
  ;[1 1 1] Capture movement
  (:Pressed
    (Variables|Movement|SetIsMovingForward true))
  (:Released
    (Variables|Movement|SetIsMovingForward false)))

(event Input|ActionEvents|InputActionMoveBackward
  (params (Key :type Key%20Structure :default "AnyKey"))
  ;[1 1 1] Capture movement
  (:Pressed
    (Variables|Movement|SetIsMovingBackward true))
  (:Released
    (Variables|Movement|SetIsMovingBackward false)))

(event Input|ActionEvents|InputActionMoveLeft
  (params (Key :type Key%20Structure :default "AnyKey"))
  ;[1 1 1] Capture movement
  (:Pressed
    (Variables|Movement|SetIsMovingLeft true))
  (:Released
    (Variables|Movement|SetIsMovingLeft false)))

(event Input|ActionEvents|InputActionMoveRight
  (params (Key :type Key%20Structure :default "AnyKey"))
  ;[1 1 1] Capture movement
  (:Pressed
    (Variables|Movement|SetIsMovingRight true))
  (:Released
    (Variables|Movement|SetIsMovingRight false)))

(event Input|ActionEvents|InputActionToggleMouse
  (params (Key :type Key%20Structure :default "AnyKey"))
  ;[1 1 1] Toggle mouse cursor visibility
  (:Pressed
    (if (Variables|/Script/Engine.PlayerController|GetbShowMouseCursor (Game|GetPlayerController 0))
      (CallFunction|HideMouseCursor)
      (else
        (CallFunction|ShowMouseCursor)))))

(event Input|MouseEvents|MouseX
  (params (AxisValue :type Float%20%28single-precision%29))
  (bind _pawn (Variables|Default|GetPawn))
  (bind _returnvalue (Transformation|GetWorldRotation _pawn))
  ;[1 1 1] Mouse pan yaw
  (if (and (Variables|Movement|GetIsPanningEnabled) (not (Variables|Picker|GetIsPickerEnabled)))
    (Transformation|SetWorldRotation _pawn (Math|Rotator|MakeRotator 0.0 (.pitch _returnvalue) (+ (.yaw _returnvalue) (* AxisValue (Variables|Config|GetPanYawSpeed)))) false false)))

(event Input|MouseEvents|MouseY
  (params (AxisValue :type Float%20%28single-precision%29))
  (bind _pawn (Variables|Default|GetPawn))
  (bind _returnvalue (Transformation|GetWorldRotation _pawn))
  ;[1 1 1] Mouse pan pitch
  (if (and (Variables|Movement|GetIsPanningEnabled) (not (Variables|Picker|GetIsPickerEnabled)))
    (Transformation|SetWorldRotation _pawn (Math|Rotator|MakeRotator 0.0 (Math|Float|Clamp(Float) (+ (* AxisValue (Variables|Config|GetPanPitchSpeed)) (.pitch _returnvalue)) -89.9 89.9) (.yaw _returnvalue)) false false)))

(fn ConstructionScript)

(fn MovePawn
  (params (Direction :type Vector) (Speed :type Float%20%28single-precision%29))
  (bind _pawn (Variables|Default|GetPawn))
  (bind _pawn_2 (Variables|Default|GetPawn))
  (bind _movementspeed (Variables|Config|GetMovementSpeed))
  (bind _returnvalue (Transformation|GetWorldTransform _pawn))
  (bind _returnvalue_2 (Math|Transform|TransformDirection _returnvalue Direction))
  (bind _returnvalue_3 (* _returnvalue_2 Speed))
  (bind _returnvalue_4 (* _returnvalue_3 _movementspeed))
  (if (Variables|Movement|GetIsMovingFast)
    (Physics|AddForce _pawn_2 (* _returnvalue_4 (Variables|Config|GetMoveFastMultiplier)) "None" false)
    (else
      (Physics|AddForce _pawn_2 _returnvalue_4 "None" false))))

(fn ShowMouseCursor
  (Variables|/Script/Engine.PlayerController|SetbShowMouseCursor (Game|GetPlayerController 0) true)
  (Variables|Movement|SetIsPanningEnabled false))

(fn HideMouseCursor
  (Variables|/Script/Engine.PlayerController|SetbShowMouseCursor (Game|GetPlayerController 0) false)
  (Variables|Movement|SetIsPanningEnabled true))

(fn EnablePicker
  (bind _camera (Variables|Default|GetCamera))
  (bind _returnvalue (Transformation|GetWorldLocation _camera))
  (bind _outhit (Collision|LineTraceByChannel _returnvalue (+ _returnvalue (* (.WorldDirection (Game|Player|ConvertMouseLocationToWorldSpace (Game|GetPlayerController 0))) (Variables|Config|GetPickerMaxDistance))) "TraceTypeQuery1" false 0 "None"))
  (if (Physics|IsSimulatingPhysics (.hitcomponent _outhit) "None")
    (Variables|Picker|SetIsPickerEnabled true)
    (Variables|Picker|SetPickedObject (.hitcomponent _outhit))
    (if (Game|Player|IsInputKeyDown (Game|GetPlayerController 0) "LeftAlt")
      (LocalVariables|SetPickupPoint (.location _outhit))
      (LocalVariables|SetShouldConstraintRotation false)
      (else
        (LocalVariables|SetPickupPoint (+ (Transformation|GetWorldLocation (.hitcomponent _outhit)) (stale _returnvalue)))
        (LocalVariables|SetShouldConstraintRotation true)))
    (Variables|Picker|SetPickDistance (Math|Vector|VectorLength (- (LocalVariables|GetPickupPoint) (Transformation|GetWorldLocation (Variables|Default|GetCamera)))))
    (Class|PhysicsHandleComponent|GrabComponent (Variables|Default|GetPhysicsHandle) (.hitcomponent _outhit) "None" (LocalVariables|GetPickupPoint) (LocalVariables|GetShouldConstraintRotation))))

(fn DisablePicker
  (if (Variables|Picker|GetIsPickerEnabled)
    (Variables|Picker|SetIsPickerEnabled false)
    (Physics|Components|PhysicsHandle|ReleaseComponent (Variables|Default|GetPhysicsHandle))
    (Class|PrimitiveComponent|WakeRigidBody (Variables|Picker|GetPickedObject) "None")))

(fn ApplyPickerForces
  (if (Variables|Picker|GetIsPickerEnabled)
    (Physics|Components|PhysicsHandle|SetTargetLocation (Variables|Default|GetPhysicsHandle) (+ (Transformation|GetWorldLocation (Variables|Default|GetCamera)) (* (.WorldDirection (Game|Player|ConvertMouseLocationToWorldSpace (Game|GetPlayerController 0))) (Variables|Picker|GetPickDistance))))))