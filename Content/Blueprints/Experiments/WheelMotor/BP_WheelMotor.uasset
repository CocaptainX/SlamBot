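; Experimental wheel motor actor whose graph holds only a readout of the Wheel component's spin speed, with no drive logic.
; Tick projects the wheel's physics angular velocity onto its local Y axis to get signed degrees per second.
; A helper function converts that value to RPM.
; The formatted debug print of both values is disconnected, so the readout never displays.
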(event `self.ReceiveBeginPlay`)

(event `self.ReceiveActorBeginOverlap`
  (params (OtherActor :type "Actor Object Reference")))

(event `self.ReceiveTick`
  (params (DeltaSeconds :type "Float (single-precision)"))
  (bind _wheel (`self.Wheel`))
  (bind _returnvalue (`PrimitiveComponent.GetPhysicsAngularVelocity` _wheel "None"))
  (bind _rotationsperminute (`self.ConvertDegreesPerSecondToRpm` (`KismetMathLibrary.Dot_VectorVector` _returnvalue (`KismetMathLibrary.TransformDirection` (`SceneComponent.K2_GetComponentToWorld` _wheel) (0.0 1.0 0.0))))))

(fn `ConvertDegreesPerSecondToRpm`
  (params (DegreesPerSecond :type "Float (double-precision)"))
  (returns (RotationsPerMinute :type "Float (double-precision)"))
  (return (* (/ DegreesPerSecond 360.0) 60.0)))

(fn `UserConstructionScript`)