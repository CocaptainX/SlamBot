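; Experimental wheel-motor actor that creates a physics constraint between a parent and a child component, with no motor drive logic in its graphs.
; The construction script adds the constraint at the scene root's relative transform, attaches it to the root's attach parent and binds MotorParent to MotorChild.
; SetConstrainedComponents only stores those two references, leaving the binding to the construction script.
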(event `self.ReceiveBeginPlay`)

(event `self.ReceiveActorBeginOverlap`
  (params (OtherActor :type "Actor Object Reference")))

(event `self.ReceiveTick`
  (params (DeltaSeconds :type "Float (single-precision)")))

(fn `SetConstrainedComponents`
  (params (Parent :type "StaticMeshComponent Object Reference") (Child :type "StaticMeshComponent Object Reference"))
  (set `self.MotorParent` Parent)
  (set `self.MotorChild` Child))

(fn `UserConstructionScript`
  (bind _returnvalue (`AddComponent|Physics Constraint Component_0` :`bManualAttachment` true :`RelativeTransform` (`SceneComponent.GetRelativeTransform` (`self.DefaultSceneRoot`))))
  (`SceneComponent.K2_AttachTo` _returnvalue (`SceneComponent.GetAttachParent` (`self.DefaultSceneRoot`)) "None" "KeepRelativeOffset" true)
  (`PhysicsConstraintComponent.SetConstrainedComponents` _returnvalue (`self.MotorParent`) "None" (`self.MotorChild`) "None"))