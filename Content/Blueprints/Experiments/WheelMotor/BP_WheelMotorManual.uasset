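; Experimental physics wheel motor that builds its constraint between Base and Wheel manually in the construction script.
; The constraint, placed at ConstraintLocation, frees twist, locks both swings and sets an angular velocity target, with high drive spring and zero damping.
; Tick projects the Wheel's angular velocity onto its local Y axis and converts it to RPM, but the debug text that would display it is disconnected.
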(event `self.ReceiveBeginPlay`)

(event `self.ReceiveActorBeginOverlap`
  (params (OtherActor :type "Actor Object Reference")))

(event `/Game/Blueprints/Experiments/WheelMotor/BP_WheelMotor.ReceiveTick`
  (params (DeltaSeconds :type "Float (single-precision)"))
  (bind _wheel (`self.Wheel`))
  (bind _returnvalue (`PrimitiveComponent.GetPhysicsAngularVelocity` _wheel "None"))
  (bind _rotationsperminute (`self.ConvertDegreesPerSecondToRpm` (`KismetMathLibrary.Dot_VectorVector` _returnvalue (`KismetMathLibrary.TransformDirection` (`SceneComponent.K2_GetComponentToWorld` _wheel) (0.0 1.0 0.0))))))

(fn `ConvertDegreesPerSecondToRpm`
  (params (DegreesPerSecond :type "Float (double-precision)"))
  (returns (RotationsPerMinute :type "Float (double-precision)"))
  (return (* (/ DegreesPerSecond 360.0) 60.0)))

(fn `UserConstructionScript`
  (bind _returnvalue (`AddComponent|Physics Constraint Component_233` :`RelativeTransform` (`SceneComponent.GetRelativeTransform` (`self.ConstraintLocation`))))
  (`|ExecutionSequence`
    (:`then_0`
      (`PhysicsConstraintComponent.SetConstrainedComponents` _returnvalue (`self.Base`) "None" (`self.Wheel`) "None"))
    (:`then_1`
      (`PhysicsConstraintComponent.SetAngularTwistLimit` _returnvalue "ACM_Free" 0.0))
    (:`then_2`
      (`PhysicsConstraintComponent.SetAngularSwing1Limit` _returnvalue "ACM_Locked" 0.0))
    (:`then_3`
      (`PhysicsConstraintComponent.SetAngularSwing2Limit` _returnvalue "ACM_Locked" 0.0))
    (:`then_4`
      (`PhysicsConstraintComponent.SetAngularVelocityDrive` _returnvalue true true))
    (:`then_5`
      (`PhysicsConstraintComponent.SetAngularVelocityTarget` _returnvalue (10.0 0.0 0.0)))
    (:`then_6`
      (`PhysicsConstraintComponent.SetAngularDriveParams` _returnvalue 1000000.0 0.0 1000000.0))))