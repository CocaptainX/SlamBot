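; BP_SlamLibrary is an experimental test Blueprint that checks whether the external Slam library DLL loads and responds.
; On BeginPlay it loads SlamLibrary.dll from the SlamLibrary folder, then calls InvertBool as a smoke test of the library.
; Each stage reports success or failure through PrintString.
; A separate TestSlam call is left unconnected and never runs.
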(event `self.ReceiveBeginPlay`
  (`KismetSystemLibrary.PrintString` "Test Slam library!")
  (bind _returnvalue (`SlamLibrary.loadSlamLibrary` "SlamLibrary"))
  (if _returnvalue
    (`KismetSystemLibrary.PrintString` "Slam library was loaded!")
    (`|ExecutionSequence`
      (:`then_0`
        (bind _returnvalue_2 (`SlamLibrary.invertBool` false))
        (if _returnvalue_2
          (`KismetSystemLibrary.PrintString` "Slam library DLL works!")
          (else
            (`KismetSystemLibrary.PrintString` "Something wrong with the Slam library DLL!")))))
    (else
      (`KismetSystemLibrary.PrintString` "Loading slam library failed!"))))

(fn `UserConstructionScript`)