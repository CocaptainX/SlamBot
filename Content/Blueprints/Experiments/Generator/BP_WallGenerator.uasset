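; BP_WallGenerator is an experimental generator that builds a wall of physics-simulated static mesh pieces.
; Its construction script runs nested column and row loops, adding a mesh component per cell with physics simulation enabled.
; The Arrow's world transform sets the origin and each piece's rotation and scale.
; Scaled spacing offsets run along world X and Z, so the grid itself does not follow the Arrow's rotation.
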(event `self.ReceiveBeginPlay`)

(fn `UserConstructionScript`
  (bind _returnvalue (`SceneComponent.K2_GetComponentToWorld` (`self.Arrow`)))
  (for _index (range (+ (`self.ColumnCount`) 1))
    (for _index_2 (range (+ (`self.RowCount`) 1))
      (bind _returnvalue_2 (`AddComponent|NODE_AddStaticMeshComponent-0` :`bManualAttachment` true))
      (`SceneComponent.K2_AttachTo` _returnvalue_2 (`self.Scene`) "None" "KeepRelativeOffset" true)
      (`StaticMeshComponent.SetStaticMesh` _returnvalue_2 (`self.StaticMesh`))
      (`PrimitiveComponent.SetSimulatePhysics` _returnvalue_2 true)
      (`SceneComponent.K2_SetWorldTransform` _returnvalue_2 (`KismetMathLibrary.MakeTransform` (`KismetMathLibrary.MakeVector` (+ (* (* _index (`self.HorizontalSpacing`)) (.x (.scale _returnvalue))) (.x (.location _returnvalue))) (.y (.location _returnvalue)) (+ (* (* _index_2 (`self.VerticalSpacing`)) (.z (.scale _returnvalue))) (.z (.location _returnvalue)))) (.rotation _returnvalue) (`KismetMathLibrary.MakeVector` (.x (.scale _returnvalue)) (.y (.scale _returnvalue)) (.z (.scale _returnvalue)))) false false))))