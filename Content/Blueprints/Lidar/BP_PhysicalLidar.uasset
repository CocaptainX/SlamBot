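; Actor that drives a physical lidar over a serial port, switching its motor on and off with play, and visualizes its scans in the world.
; Tick drains serial messages, parsing comma-separated angle, distance and signal strength into a capped FIFO of measurements.
; Each measurement rotates the origin's forward vector into a grid-snapped point, shown as a mesh instance.
; A wrapping index reuses instances once the maximum count is reached.
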(event `self.ReceiveBeginPlay`
  (bind _returnvalue (`self.OpenPort` (`self.SerialPortName`)))
  (if _returnvalue
    (`self.StartLidar`)))

(event `self.ReceiveEndPlay`
  (params (EndPlayReason :type "EEndPlayReason Enum" :default "Destroyed"))
  (if (`self.IsConnected`)
    (`self.StopLidar`)))

(event `self.ReceiveTick`
  (params (DeltaSeconds :type "Float (single-precision)"))
  (`self.ReadSerialMessages`))

(event `MeasurementReceived`
  (params (Measurement :type "/Game/Blueprints/Lidar/ST_LidarMeasurement Structure"))
  (`self.VisualizeMeasurement` Measurement))

(fn `CalculateMeasurementRelativeTransform`
  (params (Measurement :type "/Game/Blueprints/Lidar/ST_LidarMeasurement Structure"))
  (returns (RelativeTransform :type "Transform Structure"))
  (bind _snappedlocation (`self.SnapLocation` (* (`KismetMathLibrary.RotateAngleAxis` (`SceneComponent.GetForwardVector` (`self.Origin`)) (* (`KismetMathLibrary.Conv_IntToDouble` Measurement_Angle_2_C0CCD6DE449D420F3E08468B4E93501D) -1.0) (0.0 0.0 1.0)) (`KismetMathLibrary.Conv_IntToDouble` Measurement_Distance_5_3A2214D4432E471112E8F4A20809DB7F)) (`self.SnapGridSize`)))
  (return (`KismetMathLibrary.MakeTransform` _snappedlocation (`KismetMathLibrary.MakeRotator` 0.0))))

(fn `ParseDistanceMeasurement`
  (params (Message :type String))
  (locals (Measurement :type "/Game/Blueprints/Lidar/ST_LidarMeasurement Structure" :default (struct)) (IsValidMeasurement :type Boolean))
  (bind _measurement (`local.Measurement`))
  (bind (_measurement_angle _measurement_distance _measurement_signalstrength) (break `/Game/Blueprints/Lidar/ST_LidarMeasurement` (`local.Measurement`)))
  (`|ExecutionSequence`
    (:`then_0`
      ;[1 1 1] Create local measurement struct
      (set `local.Measurement` (make `/Game/Blueprints/Lidar/ST_LidarMeasurement` 0)))
    (:`then_1`
      ;[1 1 1] Parse string message to measurement struct
      (for (_array_element _array_index) (`KismetStringLibrary.ParseIntoArray` Message ",")
        (switch `int` _array_index
          (:`1`
            (setmembers `/Game/Blueprints/Lidar/ST_LidarMeasurement` :`StructRef` _measurement :`Angle` (`KismetStringLibrary.Conv_StringToInt` _array_element)))
          (:`2`
            (setmembers `/Game/Blueprints/Lidar/ST_LidarMeasurement` :`StructRef` _measurement :`Distance` (/ (`KismetStringLibrary.Conv_StringToInt` _array_element) 10)))
          (:`3`
            (bind _structout (setmembers `/Game/Blueprints/Lidar/ST_LidarMeasurement` :`StructRef` _measurement :`SignalStrength` (`KismetStringLibrary.Conv_StringToInt` _array_element)))
            ;[1 1 1] Add the valid measurement and trigger event
            (`KismetArrayLibrary.Array_Add` (`self.Measurements`) _structout)
            (`self.MeasurementReceived` _structout)))))
    (:`then_2`
      ;[1 1 1] Keep a maximum number of measurements in a FIFO
      (while (> (`KismetArrayLibrary.Array_Length` (`self.Measurements`)) (`self.MaxMeasurementCount`))
        (`KismetArrayLibrary.Array_Remove` (`self.Measurements`))))
    (:`then_3`
      ;[1 1 1] Log to console if requested
      (if (`self.UseDebugLog`)
        (`KismetSystemLibrary.PrintText` (`|FormatText` "LIDAR: {distance} at angle {angle} with strength {strength}" (`KismetTextLibrary.Conv_IntToText` _measurement_distance) (`KismetTextLibrary.Conv_IntToText` _measurement_angle) (`KismetTextLibrary.Conv_IntToText` _measurement_signalstrength)))))))

(fn `ReadSerialMessages`
  (while (> (`self.MessageCount`) 0)
    (bind _returnvalue (`self.GetNextMessage`))
    (`self.ParseDistanceMeasurement` _returnvalue)))

(fn `SnapLocation`
  (params (Location :type "Vector Structure") (GridSize :type Integer))
  (returns (SnappedLocation :type "Vector Structure"))
  (bind _returnvalue (`KismetMathLibrary.Conv_IntToDouble` GridSize))
  (return (`KismetMathLibrary.MakeVector` (`KismetMathLibrary.Conv_IntToDouble` (* (`KismetMathLibrary.Round` (/ Location_X _returnvalue)) GridSize)) (`KismetMathLibrary.Conv_IntToDouble` (* (`KismetMathLibrary.Round` (/ Location_Y _returnvalue)) GridSize)) (`KismetMathLibrary.Conv_IntToDouble` (* (`KismetMathLibrary.Round` (/ Location_Z _returnvalue)) GridSize)))))

(fn `StartLidar`
  (`self.SendMessage` "MotorOn" true))

(fn `StopLidar`
  (`self.SendMessage` "MotorOff" true))

(fn `UserConstructionScript`)

(fn `VisualizeMeasurement`
  (params (Measurement :type "/Game/Blueprints/Lidar/ST_LidarMeasurement Structure"))
  (bind _visualizationmeshes (`self.VisualizationMeshes`))
  (`|ExecutionSequence`
    (:`then_0`
      (bind _relativetransform (`self.CalculateMeasurementRelativeTransform` Measurement))
      (if (< (`InstancedStaticMeshComponent.GetInstanceCount` _visualizationmeshes) (`self.MaxMeasurementCount`))
        (`InstancedStaticMeshComponent.AddInstance` _visualizationmeshes _relativetransform)
        (else
          (`InstancedStaticMeshComponent.UpdateInstanceTransform` _visualizationmeshes (`self.VisualMeasurementIndex`) _relativetransform false true false))))
    (:`then_1`
      (set `self.VisualMeasurementIndex` (mod (+ (`self.VisualMeasurementIndex`) 1) (`self.MaxMeasurementCount`))))))